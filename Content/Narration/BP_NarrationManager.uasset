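; Narration manager that shows narration sequences and handles what follows when they end.
; DisplayNarration blocks player inputs, switches input mode and launches a WBP_Narration widget through its interface, with InteractonNarration forwarding skips to it.
; On scene end, it either calls Transition on BP_TransitionLVL, or restores input, removes the widget and has BP_SceneManager change to NextLevel at TargetID, depending on the AddTransitionLvl flag.
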(event `self.ReceiveBeginPlay`
  (bind _returnvalue (`GameplayStatics.GetActorOfClass` "/Game/SceneManagement/BP_SceneManager.BP_SceneManager_C"))
  (set `self.SceneManager` _returnvalue))

(event `/Game/Narration/BPI_NarrationManager.DisplayNarration`
  (params (RowName :type Name) (isNarrationScene :type Boolean) (addTransitionLvl :type Boolean))
  (bind _returnvalue (`GameplayStatics.GetPlayerController` 0))
  ;[1 1 1] Creation widget
  (set `self.Add Transition Lvl` addTransitionLvl)
  (message `/Game/Player/BPI_PlayerController.BlockPlayerInputs` _returnvalue "NewEnumerator2")
  (message `/Game/Player/BPI_PlayerController.SetPlayerInputMode` _returnvalue "NewEnumerator4")
  (bind _returnvalue_2 (`|CreateWidget` "/Game/Narration/WBP_Narration.WBP_Narration_C"))
  (bind _output_get (set `self.CurrentWidget` _returnvalue_2))
  (if (`KismetSystemLibrary.DoesImplementInterface` _returnvalue_2 "/Game/Narration/BPI_WBP_Narration.BPI_WBP_Narration_C")
    (message `/Game/Narration/BPI_WBP_Narration.LaunchDisplayNarration` _output_get RowName isNarrationScene)
    (`UserWidget.AddToViewport` _output_get 0)
    (else
      ;;[1 0 0 0.33] Error
      (`KismetSystemLibrary.PrintString` "ERROR: Interface missing in WBP_Narration" true true (struct :`R` 1.0 :`A` 1.0) 12000.0))))

(event `/Game/Narration/BPI_NarrationManager.InteractOnNarration`
  (bind _currentwidget (`self.CurrentWidget`))
  ;[1 1 1] Interaction from PlayerController
  (`/Engine/EditorBlueprintResources/StandardMacros.IsValid` _currentwidget
    (:`Is Valid`
      (message `/Game/Narration/BPI_WBP_Narration.Skip` _currentwidget))))

(event `/Game/Narration/BPI_NarrationManager.EndSceneNarration`
  (bind _returnvalue (`GameplayStatics.GetPlayerController` 0))
  (bind _next_level (`self.Next Level`))
  ;[1 1 1] End Narration scene
  (if (not (`self.Add Transition Lvl`))
    (message `/Game/Player/BPI_PlayerController.UnblockPlayerInputs` _returnvalue "NewEnumerator2")
    (message `/Game/Player/BPI_PlayerController.SetPlayerInputMode` _returnvalue "NewEnumerator0")
    (`Widget.RemoveFromParent` (`self.CurrentWidget`))
    (if (`KismetSystemLibrary.IsValidSoftObjectReference` _next_level)
      (`/Game/SceneManagement/BP_SceneManager.ChangeLevel` (`self.SceneManager`) _next_level (`self.TargetID`) true false)
      (else
        ;;[1 0 0 0.33] Error: scene ref empty
        (`KismetSystemLibrary.PrintString` "Error: Target scene not valid" true true (struct :`R` 1.0 :`A` 1.0) 12000.0)))
    (else
      (bind _returnvalue_2 (`GameplayStatics.GetActorOfClass` "/Game/SceneManagement/BP_TransitionLVL.BP_TransitionLVL_C"))
      (`/Game/SceneManagement/BP_TransitionLVL.Transition` _returnvalue_2))))

(fn `UserConstructionScript`)