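; BP_RotationSupport is a gameplay element actor that rotates around its yaw axis by a given angle over a given duration.
; StartRotation ignores calls while already rotating, otherwise derives a constant speed, and Tick sets yaw from the start angle and clamped elapsed time.
; Registered child rotatables are notified when rotation starts and stops.
; It also exposes its current angle and a range derived from the RotationBase's X scale.
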(event `self.ReceiveBeginPlay`
  (bind (_returnvalue_roll _returnvalue_pitch _returnvalue_yaw) (`KismetMathLibrary.BreakRotator` (`self.K2_GetActorRotation`)))
  (set `self.InnerRotation` _returnvalue_yaw))

(event `self.ReceiveTick`
  (params (DeltaSeconds :type "Float (single-precision)"))
  (bind (_returnvalue_roll _returnvalue_pitch) (`KismetMathLibrary.BreakRotator` (`self.K2_GetActorRotation`)))
  (if (`self.bIsRotating`)
    (`|ExecutionSequence`
      (:`then_0`
        (bind _output_get (set `self.InnerRotationTimer` (+ (`self.InnerRotationTimer`) DeltaSeconds)))
        (if (>= _output_get (`self.InnerRotationEndTime`))
          (set `self.InnerRotationTimer` (`self.InnerRotationEndTime`))
          (set `self.bIsRotating` false)
          (`self.StopRotationOnChildrens`)))
      (:`then_1`
        (bind _output_get_2 (set `self.InnerRotation` (mod (+ (`self.InnerRotationAtStart`) (* (`self.InnerRotationSpeed`) (`self.InnerRotationTimer`))) 360.0)))
        (`self.K2_SetActorRotation` (`KismetMathLibrary.MakeRotator` _returnvalue_roll _returnvalue_pitch _output_get_2))))))

(fn `AddRotatatble`
  (params (Rotatable :type "/Game/SceneManagement/SceneRotation/BPAC_SceneRotationObject Object Reference"))
  (`KismetArrayLibrary.Array_AddUnique` (`self.ChildsRotatable`) Rotatable))

(fn `Get RotationAngle`
  (returns (RotationAngle :type "Float (double-precision)"))
  (return (`self.InnerRotation`)))

(fn `GetRange`
  (returns (Range :type "Float (double-precision)"))
  (bind _returnvalue_x (`KismetMathLibrary.BreakVector` (`SceneComponent.K2_GetComponentScale` (`self.RotationBase`))))
  (return (* _returnvalue_x 50.0)))

(fn `StartRotation`
  (params (RotationAngle :type "Float (double-precision)") (RotationDuration :type "Float (double-precision)"))
  (bind (_returnvalue_roll _returnvalue_pitch _returnvalue_yaw) (`KismetMathLibrary.BreakRotator` (`self.K2_GetActorRotation`)))
  (if (not (`self.bIsRotating`))
    (set `self.bIsRotating` true)
    (set `self.InnerRotationSpeed` (/ RotationAngle RotationDuration))
    (set `self.InnerRotationEndTime` RotationDuration)
    (set `self.InnerRotationTimer` 0.0)
    (set `self.InnerRotationAtStart` _returnvalue_yaw)
    (`self.StartRotationOnChildrens`)
    (`KismetSystemLibrary.PrintText` "Starting Debug Rotation on a Rotation Support." true true (struct :`R` 0.237686 :`G` 1.0 :`A` 1.0) 2.0 "Debug Rotation Log")
    (else
      (`KismetSystemLibrary.PrintText` "The Rotation Support selected for Debug Rotation is already rotating." true true (struct :`R` 1.0 :`G` 0.077466 :`A` 1.0) 2.0 "Debug Rotation Log"))))

(fn `StartRotationOnChildrens`
  (for _array_element (`self.ChildsRotatable`)
    (`/Game/SceneManagement/SceneRotation/BPAC_SceneRotationObject.SetRotating` _array_element true)))

(fn `StopRotationOnChildrens`
  (if (not (`self.bIsRotating`))
    (for _array_element (`self.ChildsRotatable`)
      (`/Game/SceneManagement/SceneRotation/BPAC_SceneRotationObject.SetRotating` _array_element false))))

(fn `UserConstructionScript`)