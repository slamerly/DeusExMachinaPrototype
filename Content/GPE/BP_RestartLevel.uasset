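; BP_RestartLevel is a trigger volume that restarts the game by reloading LVL_GTP_Main when the player enters it.
; Box overlap by a BPC_Player_CameraTest shows that player's FadeBlack widget, plays CameraEyesSeeYouFade, then opens the level after a short delay.
; The sequence requires the game mode to cast to GameMode or, failing that, GM_TestCam.
; A branch that would hide the fade again is left unconnected.
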(event `self.Box.OnComponentBeginOverlap`
  (params (OverlappedComponent :type "PrimitiveComponent Object Reference") (OtherActor :type "Actor Object Reference") (OtherComp :type "PrimitiveComponent Object Reference") (OtherBodyIndex :type Integer) (bFromSweep :type Boolean) (SweepResult :type "HitResult Structure (by ref)"))
  (bind _asbpc_player_camera_test (cast `/Game/Player/BPC_Player_CameraTest` OtherActor))
  (cast `GameMode` (`GameplayStatics.GetGameMode`)
    (:`then`
      _)
    (:`CastFailed`
      (cast `/Game/_GameManager/GM_TestCam` (`GameplayStatics.GetGameMode`))))
  (bind _widgetfadeblack (`/Game/Player/BPC_Player_CameraTest.WidgetFadeBlack` _asbpc_player_camera_test))
  (`Widget.SetVisibility` (`/Game/Widget/WBP_FadeBlack.FadeBlack` _widgetfadeblack) "Visible")
  (`/Game/Widget/WBP_FadeBlack.CameraEyesSeeYouFade` _widgetfadeblack)
  (`KismetSystemLibrary.Delay` 1.5)
  (`GameplayStatics.OpenLevel` "LVL_GTP_Main"))

(fn `UserConstructionScript`)