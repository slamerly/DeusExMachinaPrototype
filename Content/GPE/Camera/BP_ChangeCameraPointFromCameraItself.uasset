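; Camera trigger that switches the player camera's view target when the camera's own collision enters its collider.
; A FlipFlop alternates entries between next and previous camera points with their interp speeds, behind a DoOnce re-armed on overlap end.
; Entry also opens a Tick gate that, if enabled, eases the camera's distance threshold toward an offset.
; The return pass overwrites that offset with the previous value, which the forward pass never restores.
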(event `self.ReceiveBeginPlay`
  (bind _asbpc_player_camera_test (cast `/Game/Player/BPC_Player_CameraTest` (`GameplayStatics.GetPlayerPawn` 0)))
  (set `self.As BPC Player Camera Test` _asbpc_player_camera_test))

(event `self.ReceiveTick`
  (params (DeltaSeconds :type "Float (single-precision)"))
  (bind _as_bpc_player_camera_test (`self.As BPC Player Camera Test`))
  (if (and (`self.OpenEventTick`) (`self.ApplyCameraDistanceOffset`))
    (bind _output_get (set `/Game/Player/BPC_Player_CameraTest.DistanceFromPlayerThreshold` (`KismetMathLibrary.FInterpTo` (`/Game/Player/BPC_Player_CameraTest.DistanceFromPlayerThreshold` _as_bpc_player_camera_test) (`self.CameraDistanceOffset`) (`GameplayStatics.GetWorldDeltaSeconds`) (`self.Interp Speed Threshold`)) _as_bpc_player_camera_test))
    (if (`KismetMathLibrary.NearlyEqual_FloatFloat` _output_get (`self.CameraDistanceOffset`) 1.0)
      (set `self.OpenEventTick` false))))

(event `self.Collider Switch.OnComponentBeginOverlap`
  (params (OverlappedComponent :type "PrimitiveComponent Object Reference") (OtherActor :type "Actor Object Reference") (OtherComp :type "PrimitiveComponent Object Reference") (OtherBodyIndex :type Integer) (bFromSweep :type Boolean) (SweepResult :type "HitResult Structure (by ref)"))
  (bind _as_bpc_player_camera_test (`self.As BPC Player Camera Test`))
  (bind _as_bpc_player_camera_test_2 (`self.As BPC Player Camera Test`))
  (if (== OtherComp (`/Game/Player/BPC_Player_CameraTest.CameraCollision` (`self.As BPC Player Camera Test`)))
    (set `self.OpenEventTick` true)
    (`/Engine/EditorBlueprintResources/StandardMacros.DoOnce` false :!label _label
      (:`Completed`
        (`/Engine/EditorBlueprintResources/StandardMacros.FlipFlop`
          (:`A`
            (set `/Game/Player/BPC_Player_CameraTest.CameraViewTarget` (`self.NextCameraPoint`) _as_bpc_player_camera_test_2)
            (set `/Game/Player/BPC_Player_CameraTest.Interp Speed Rotation Camera` (`self.Interp Speed Rotation Camera Reference`) _as_bpc_player_camera_test_2)
            (set `/Game/Player/BPC_Player_CameraTest.DistanceOnSplineInterpSpeed` (`self.Distance On Spline Interp Speed Reference`) _as_bpc_player_camera_test_2))
          (:`B`
            (set `/Game/Player/BPC_Player_CameraTest.CameraViewTarget` (`self.PreviousCameraPoint`) _as_bpc_player_camera_test)
            (set `/Game/Player/BPC_Player_CameraTest.Interp Speed Rotation Camera` (`self.Previous Interp Speed Rotation`) _as_bpc_player_camera_test)
            (set `self.CameraDistanceOffset` (`self.PreviousCameraDistanceOffset`))
            (set `/Game/Player/BPC_Player_CameraTest.DistanceOnSplineInterpSpeed` (`self.Previous Distance On Spline Interp Speed Reference`) _as_bpc_player_camera_test)))))))

(event `self.Collider Switch.OnComponentEndOverlap`
  (params (OverlappedComponent :type "PrimitiveComponent Object Reference") (OtherActor :type "Actor Object Reference") (OtherComp :type "PrimitiveComponent Object Reference") (OtherBodyIndex :type Integer))
  (goto _label :!via `Reset`))

(fn `UserConstructionScript`)