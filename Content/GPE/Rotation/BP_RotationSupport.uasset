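; Rotating platform that turns on yaw through a curve-driven timed rotation, with a failed-rotation variant and a toggleable outline.
; StartRotation rejects overlapping requests, Tick animates the yaw, and registered rotatables receive start and stop states.
; Supports nest through their own BPAC_RotatableObject, which defers the children's stop and defines the upper layer, falling back to RotationSceneManager.
; UpdateTesting previews angles by finding attached rotatables and propagating the rotation to them.
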(event `self.ReceiveBeginPlay`
  (bind (_returnvalue_roll _returnvalue_pitch _returnvalue_yaw) (`KismetMathLibrary.BreakRotator` (`self.K2_GetActorRotation`)))
  (bind (_returnvalue_x _returnvalue_y) (`KismetMathLibrary.BreakVector` (`SceneComponent.K2_GetComponentScale` (`self.RotationBase`))))
  (`|ExecutionSequence`
    (:`then_0`
      (bind _output_get (set `self.BeginPlayRotation` _returnvalue_yaw))
      (set `self.InnerRotation` _output_get))
    (:`then_1`
      (`SceneComponent.SetWorldScale3D` (`self.Outline`) (`KismetMathLibrary.MakeVector` (+ _returnvalue_x 0.1) (+ _returnvalue_y 0.1) 0.01)))))

(event `self.ReceiveTick`
  (params (DeltaSeconds :type "Float (single-precision)"))
  (bind (_returnvalue_roll _returnvalue_pitch) (`KismetMathLibrary.BreakRotator` (`self.K2_GetActorRotation`)))
  (if (`self.bIsRotating`)
    (`|ExecutionSequence`
      (:`then_0`
        (bind _output_get (set `self.InnerRotationTimer` (+ (`self.InnerRotationTimer`) DeltaSeconds)))
        (if (>= _output_get (`self.InnerRotationEndTime`))
          (set `self.InnerRotationTimer` (`self.InnerRotationEndTime`))
          (set `self.bIsRotating` false)
          (`self.StopRotationOnChildrens`)))
      (:`then_1`
        (bind _output_get_2 (set `self.InnerRotation` (mod (+ (`self.InnerRotationAtStart`) (* (`CurveFloat.GetFloatValue` (`self.InnerRotationCurve`) (/ (`self.InnerRotationTimer`) (`self.InnerRotationEndTime`))) (`self.InnerRotationAngle`))) 360.0)))
        (`self.K2_SetActorRotation` (`KismetMathLibrary.MakeRotator` _returnvalue_roll _returnvalue_pitch _output_get_2))))))

(fn `ActualiseTestingAngle`
  (`self.UpdateTesting` false true))

(fn `AddRotatatble`
  (params (Rotatable :type "/Game/GPE/Rotation/BPAC_RotatableObject Object Reference"))
  (`KismetArrayLibrary.Array_AddUnique` (`self.ChildsRotatable`) Rotatable))

(fn `Get RotationAngle`
  (returns (RotationAngle :type "Float (double-precision)"))
  (return (`self.InnerRotation`)))

(fn `GetLayerName`
  (returns (Name :type String))
  (return (`KismetStringLibrary.Concat_StrStr` (`KismetSystemLibrary.GetDisplayName` self) " Layer")))

(fn `GetObject`
  (returns (Object :type "Actor Object Reference"))
  (return self))

(fn `GetRange`
  (returns (Range :type "Float (double-precision)"))
  (bind _returnvalue_x (`KismetMathLibrary.BreakVector` (`SceneComponent.K2_GetComponentScale` (`self.RotationBase`))))
  (return (+ (* _returnvalue_x 50.0) 50.0)))

(fn `GetRotationAngleOffsetBeginPlay`
  (returns (`Angle Offset` :type "Float (double-precision)"))
  (return (- (`self.InnerRotation`) (`self.BeginPlayRotation`))))

(fn `GetUpperLayer`
  (returns (UpperLayerExists :type Boolean) (UpperLayer :type "/Game/SceneManagement/SceneRotation/BPI_RotationLayerParent Interface"))
  (bind (_isrotatable _rotatablecomp) (`self.IsRotatable`))
  (if _isrotatable
    (return true (`/Game/GPE/Rotation/BPAC_RotatableObject.RotationSupport` _rotatablecomp))
    (else
      (return true (`self.RotationSceneManager`)))))

(fn `IsRotatable`
  (returns (IsRotatable :type Boolean) (RotatableComp :type "/Game/GPE/Rotation/BPAC_RotatableObject Object Reference"))
  (bind _returnvalue (`self.GetComponentByClass` "/Game/GPE/Rotation/BPAC_RotatableObject.BPAC_RotatableObject_C"))
  (`/Engine/EditorBlueprintResources/StandardMacros.IsValid` _returnvalue
    (:`Is Valid`
      (if (`/Game/GPE/Rotation/BPAC_RotatableObject.IsRotatableValid` _returnvalue)
        (return true _returnvalue)
        (else
          _)))
    (:`Is Not Valid`
      _))
  (return false null))

(fn `SetOutlineVisibility`
  (params (Visibility :type Boolean))
  (`SceneComponent.SetVisibility` (`self.Outline`) Visibility false))

(fn `StartFailedRotation`
  (params (FailedRotationToLeft :type Boolean))
  (bind _failrotamplitude (`self.FailRotAmplitude`))
  (if (not (`self.bIsRotating`))
    (`self.StartRotation` (`KismetMathLibrary.SelectFloat` (* -1.0 _failrotamplitude) _failrotamplitude FailedRotationToLeft) (`self.FailRotDuration`) (`self.FailRotCurve`))))

(fn `StartRotation`
  (params (RotationAngle :type "Float (double-precision)") (RotationDuration :type "Float (double-precision)") (RotationCurve :type "CurveFloat Object Reference"))
  (returns (RotationStarting :type Boolean))
  (bind (_returnvalue_roll _returnvalue_pitch _returnvalue_yaw) (`KismetMathLibrary.BreakRotator` (`self.K2_GetActorRotation`)))
  (if (not (`self.bIsRotating`))
    (set `self.bIsRotating` true)
    (set `self.InnerRotationAngle` RotationAngle)
    (set `self.InnerRotationEndTime` RotationDuration)
    (set `self.InnerRotationCurve` RotationCurve)
    (set `self.InnerRotationTimer` 0.0)
    (set `self.InnerRotationAtStart` _returnvalue_yaw)
    (`self.StartRotationOnChildrens`)
    (`KismetSystemLibrary.PrintText` "Starting Debug Rotation on a Rotation Support." true true (struct :`R` 0.237686 :`G` 1.0 :`A` 1.0) 2.0 "Debug Rotation Log")
    (return true)
    (else
      (`KismetSystemLibrary.PrintText` "The Rotation Support selected for Debug Rotation is already rotating." true true (struct :`R` 1.0 :`G` 0.077466 :`A` 1.0) 2.0 "Debug Rotation Log")
      (return false))))

(fn `StartRotationOnChildrens`
  (for _array_element (`self.ChildsRotatable`)
    (`/Game/GPE/Rotation/BPAC_RotatableObject.SetRotating` _array_element true)))

(fn `StopRotationOnChildrens`
  (bind _returnvalue (`self.GetComponentByClass` "/Game/GPE/Rotation/BPAC_RotatableObject.BPAC_RotatableObject_C"))
  (if (not (`self.bIsRotating`))
    (`/Engine/EditorBlueprintResources/StandardMacros.IsValid` _returnvalue
      (:`Is Valid`
        (if (not (`/Game/GPE/Rotation/BPAC_RotatableObject.IsRotating` _returnvalue))
          (for _array_element (`self.ChildsRotatable`) :!label _label
            (`/Game/GPE/Rotation/BPAC_RotatableObject.SetRotating` _array_element false))))
      (:`Is Not Valid`
        (goto _label)))))

(fn `UpdateTesting`
  (params (FromBeginPlay :type Boolean) (ComeFromSelf :type Boolean) (FuturePosIfInherited :type "Vector Structure"))
  (locals (RotatablesAttached :type "Array of /Game/GPE/Rotation/BPAC_RotatableObject Object Reference") (TestingStartAngle :type "Float (double-precision)"))
  (bind (_returnvalue_roll _returnvalue_pitch _returnvalue_yaw) (`KismetMathLibrary.BreakRotator` (`self.K2_GetActorRotation`)))
  (bind (_returnvalue_roll_2 _returnvalue_pitch_2) (`KismetMathLibrary.BreakRotator` (`self.K2_GetActorRotation`)))
  (`|ExecutionSequence`
    (:`then_0`
      (bind _outactors (`GameplayStatics.GetAllActorsOfClass` "/Script/Engine.Actor"))
      (for _array_element _outactors
        (bind _returnvalue (`self.GetComponentByClass` _array_element "/Game/GPE/Rotation/BPAC_RotatableObject.BPAC_RotatableObject_C"))
        (`/Engine/EditorBlueprintResources/StandardMacros.IsValid` _returnvalue
          (:`Is Valid`
            (if (== (`/Game/GPE/Rotation/BPAC_RotatableObject.RotationSupport` _returnvalue) self)
              (`KismetArrayLibrary.Array_AddUnique` (`local.RotatablesAttached`) _returnvalue)
              (set `local.TestingStartAngle` _returnvalue_yaw))))))
    (:`then_1`
      (if ComeFromSelf
        (`self.K2_SetActorRotation` (`KismetMathLibrary.MakeRotator` _returnvalue_roll_2 _returnvalue_pitch_2 (`self.TestingAngle`)))
        (for _array_element_2 (`local.RotatablesAttached`)
          (`/Game/GPE/Rotation/BPAC_RotatableObject.UpdateTestingRotation` _array_element_2 (- (`self.TestingAngle`) (`local.TestingStartAngle`))))
        (else
          (for _array_element_3 (`local.RotatablesAttached`)
            (`/Game/GPE/Rotation/BPAC_RotatableObject.UpdateTestingRotationFromSub` _array_element_3 FuturePosIfInherited)))))))

(fn `UserConstructionScript`)