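; Test interactable actor that toggles its Sphere's visibility on interaction and persists that state through the save system.
; BPAC_Saver's save and load events write and restore the flag in BP_SaveScene's Test map, keyed by ActorGuid.
; The construction script copies ActorGuid into ID, and CanInteract always returns true.
; A debug key (H) prints every saved visibility value from the saver's referenced save.
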(event OnSave(BPAC_Saver)
  (params (SaveGame :type Save%20Game%20Object%20Reference))
  (bind _actorguid (Variables|Default|GetActorGuid))
  ;[1 1 1] Save
  (bind _asbp_save_scene (Utilities|Casting|CastToBP_SaveScene SaveGame))
  (if (.ReturnValue (Utilities|Map|Find (.test (Variables|/Game/Save/BP_SaveScene.BP_SaveScene_C|GetStructScene _asbp_save_scene)) (Variables|Default|GetActorGuid)))
    (Utilities|Map|Remove (.test (Variables|/Game/Save/BP_SaveScene.BP_SaveScene_C|GetStructScene _asbp_save_scene)) _actorguid))
  (Utilities|Map|Add (.test (Variables|/Game/Save/BP_SaveScene.BP_SaveScene_C|GetStructScene _asbp_save_scene)) _actorguid (Utilities|Struct|MakeSTR_SaveTest (Variables|Save|GetSaveVisibitySphere))))

(event OnLoad(BPAC_Saver)
  (params (SaveGame :type Save%20Game%20Object%20Reference))
  ;[1 1 1] Load
  (bind _asbp_save_scene (Utilities|Casting|CastToBP_SaveScene SaveGame))
  (if (.ReturnValue (Utilities|Map|Find (.test (Variables|/Game/Save/BP_SaveScene.BP_SaveScene_C|GetStructScene _asbp_save_scene)) (Variables|Default|GetActorGuid)))
    (bind _output_get (Variables|Save|SetSaveVisibitySphere (.spherevisibility (.Value (Utilities|Map|Find (.test (Variables|/Game/Save/BP_SaveScene.BP_SaveScene_C|GetStructScene _asbp_save_scene)) (Variables|Default|GetActorGuid))))))
    (Rendering|SetVisibility (Variables|Default|GetSphere) _output_get false)))

(event EventBeginPlay)

(event EventInteraction
  (bind _sphere (Variables|Default|GetSphere))
  (bind _bisinteractable (CallFunction|CanInteract))
  (if _bisinteractable
    (if (Variables|Save|GetSaveVisibitySphere)
      (bind _output_get (Variables|Save|SetSaveVisibitySphere false))
      (Rendering|SetVisibility _sphere _output_get false)
      (else
        (bind _output_get_2 (Variables|Save|SetSaveVisibitySphere true))
        (Rendering|SetVisibility _sphere _output_get_2 false)))))

(event Input|KeyboardEvents|DebugKeyH
  (params (Key :type Key%20Structure :default "None") (ActionValue :type Input%20Action%20Value%20Structure))
  (:Pressed
    (bind _asbp_save_scene (Utilities|Casting|CastToBP_SaveScene (Variables|/Game/Save/BPAC_Saver.BPAC_Saver_C|GetRefSave (Variables|Default|GetBPAC_Saver))))
    (bind _values (Utilities|Map|Values (.test (Variables|/Game/Save/BP_SaveScene.BP_SaveScene_C|GetStructScene _asbp_save_scene))))
    (for _array_element _values
      (Development|PrintString (Utilities|String|ToString(Boolean) (.spherevisibility _array_element)) true true "(R=0.000000,G=1.000000,B=0.297444,A=1.000000)"))))

(fn ConstructionScript
  (Variables|Default|SetID (Variables|Default|GetActorGuid)))

(fn CanInteract
  (return true))