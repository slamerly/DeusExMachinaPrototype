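; Rotating support gameplay element that turns its base around yaw and moves the objects attached to it.
; Tick runs a state machine for curve-timed standard or failed turns, controlled turns with eased start and optional snap finish, and constant automatic spin.
; Each step updates accumulated and wrapped angles, then applies the inner transform.
; BPAC_Saver persists angles per actor, resolving mid-turn saves to start or end, while SupportValues drives clamp markers.
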(event `self.ReceiveBeginPlay`
  (bind (_returnvalue_x _returnvalue_y) (`KismetMathLibrary.BreakVector` (`SceneComponent.K2_GetComponentScale` (`self.RotationBase`))))
  (bind (_relativerotation_roll _relativerotation_pitch _relativerotation_yaw) (`KismetMathLibrary.BreakRotator` (`SceneComponent.RelativeRotation` (`self.RotationBase`))))
  (`parent.ReceiveBeginPlay`)
  (`|ExecutionSequence`
    (:`then_0`
      (bind _output_get (set `self.InnerRotation` _relativerotation_yaw))
      (set `self.AccumulatedRotation` _output_get))
    (:`then_1`
      ;[1 0.8026 0.1824] Setup Outline scale
      (`SceneComponent.SetWorldScale3D` (`self.Outline`) (`KismetMathLibrary.MakeVector` (+ _returnvalue_x 0.1) (+ _returnvalue_y 0.1) 0.01))
      (`self.UpdateClampVisual`))))

(event `self.BPAC_Saver.OnSave`
  (params (SaveGame :type "SaveGame Object Reference"))
  (bind (_angletosave _accumulatedtosave) (`self.GetRotAngleToSave`))
  ;[0.6745 1 0.4039] Save Rotation Angle
  (bind _asbp_save_scene (cast `/Game/Save/BP_SaveScene` SaveGame))
  (`BlueprintMapLibrary.Map_Add` (`.RotationSupports_37_D2B416C5427C7E7328625B9B8F040FF0` (break `/Game/Save/Timeline/STR_Scene` (`/Game/Save/BP_SaveScene.StructScene` _asbp_save_scene))) (`self.ActorGuid`) (make `/Game/Save/StructsSave/STR_Save_MovingObject` _angletosave _accumulatedtosave)))

(event `self.BPAC_Saver.OnLoad`
  (params (SaveGame :type "SaveGame Object Reference"))
  ;[0.6745 1 0.4039] Load Rotation Angle
  (`KismetSystemLibrary.DelayUntilNextTick`)
  (bind _asbp_save_scene (cast `/Game/Save/BP_SaveScene` SaveGame))
  (bind (_value _returnvalue) (`BlueprintMapLibrary.Map_Find` (`.RotationSupports_37_D2B416C5427C7E7328625B9B8F040FF0` (break `/Game/Save/Timeline/STR_Scene` (`/Game/Save/BP_SaveScene.StructScene` _asbp_save_scene))) (`self.ActorGuid`)))
  (if _returnvalue
    (bind (_rotationangle _accumulatedrotation) (break `/Game/Save/StructsSave/STR_Save_MovingObject` _value))
    (set `self.InnerRotation` _rotationangle)
    (set `self.AccumulatedRotation` _accumulatedrotation)
    (`self.SetInnerTransform`)
    (`self.AppliedInnerMovement` (`self.RotationBase`))
    (if (`self.bIsSelfMovable`)
      (`/Game/GPE/Moving/BPAC_MovableObject.ApplyMovement` (`self.SelfMovable`)))
    (`KismetSystemLibrary.DelayUntilNextTick`)
    (`self.UpdateChildsLoadScene`)))

(event `self.ReceiveTick`
  (params (DeltaSeconds :type "Float (single-precision)"))
  (`|ExecutionSequence`
    (:`then_0`
      (switch `/Game/GPE/Moving/Rotation/E_RotationState` (`self.CurrentRotationState`)
        (:`NewEnumerator1`
          ;[0.8962 1 0.8122] Compute Rotation (standard)
          (`|ExecutionSequence`
            (:`then_0`
              (bind _output_get (set `self.StandardRotationTimer` (+ (`self.StandardRotationTimer`) DeltaSeconds)))
              (if (>= _output_get (`self.StandardRotationEndTime`))
                (set `self.StandardRotationTimer` (`self.StandardRotationEndTime`))
                (`self.EndStandardRotation`)))
            (:`then_1`
              (`self.SetRotationInner` (- (+ (`self.InnerRotationAtStart`) (* (`CurveFloat.GetFloatValue` (`self.StandardRotationCurve`) (/ (`self.StandardRotationTimer`) (`self.StandardRotationEndTime`))) (`self.StandardRotationAngle`))) (`self.AccumulatedRotation`)))
              (`self.SetInnerTransform`)
              (`self.AppliedInnerMovement` (`self.RotationBase`)))))
        (:`NewEnumerator2`
          ;[0.898 1 0.5765] Compute Rotation (controlled)
          (`|ExecutionSequence`
            (:`then_0`
              (set `self.ControlledRotStartupTimer` (+ (`self.ControlledRotStartupTimer`) DeltaSeconds)))
            (:`then_1`
              (`self.SetRotationInner` (* (`CurveFloat.GetFloatValue` (`self.ControlledRotStartupCurve`) (/ (`self.ControlledRotStartupTimer`) (`self.ControlledRotStartupTime`))) (`self.ControlledRotSpeed`) DeltaSeconds))
              (`self.SetInnerTransform`)
              (`self.AppliedInnerMovement` (`self.RotationBase`)))))
        (:`NewEnumerator3`
          ;[0.725 0.8871 1] Compute Rotation (automatic)
          (`self.SetRotationInner` (* (`self.AutomaticRotationSpeed`) DeltaSeconds))
          (`self.SetInnerTransform`)
          (`self.AppliedInnerMovement` (`self.RotationBase`)))
        (:`NewEnumerator4`
          ;[0.898 1 0.5765] Compute Rotation (controlled finishing)
          (`|ExecutionSequence`
            (:`then_0`
              (bind _output_get_2 (set `self.ControlledRotFinishTimer` (+ (`self.ControlledRotFinishTimer`) DeltaSeconds)))
              (if (>= _output_get_2 (`self.ControlledRotFinishTime`))
                (set `self.ControlledRotFinishTimer` (`self.ControlledRotFinishTime`))
                (`self.StopControlledRotation` false)))
            (:`then_1`
              (`self.SetRotationInner` (- (`KismetMathLibrary.Lerp` (`self.ControlledRotSnapAngle`) (`self.InnerAtControlFinish`) (`CurveFloat.GetFloatValue` (`self.ControlledRotFinishCurve`) (/ (`self.ControlledRotFinishTimer`) (`self.ControlledRotFinishTime`)))) (`self.AccumulatedRotation`)))
              (`self.SetInnerTransform`)
              (`self.AppliedInnerMovement` (`self.RotationBase`)))))))))

(fn `ApplyTestingValues`
  (bind _rotationbase (`self.RotationBase`))
  (bind (_relativerotation_roll _relativerotation_pitch) (`KismetMathLibrary.BreakRotator` (`SceneComponent.RelativeRotation` _rotationbase)))
  (bind _output_get (set `self.TestingAngle` (`self.ModuloAngle` (`self.TestingAngle`))))
  (`self.ComputeChildsOffsetEditor`)
  (`SceneComponent.K2_SetRelativeRotation` _rotationbase (`KismetMathLibrary.MakeRotator` _relativerotation_roll _relativerotation_pitch _output_get) false false)
  (`self.ApplyChildsTestingEditor`))

(fn `ChangeRotSupportValues`
  (params (NewValues :type "/Game/GPE/Moving/Rotation/PDA_RotSupportValues Object Reference"))
  (set `self.SupportValues` NewValues)
  (`self.OnRotSupportValuesChanged`)
  (`self.UpdateClampVisual`))

(fn `EndStandardRotation`
  (`self.CheckRotationState` "NewEnumerator1"
    (:`True`
      (set `self.CurrentRotationState` "NewEnumerator0")
      (set `self.bIsInFailedRot` false)
      (`self.StopMovementOnChildrens`))))

(fn `ForceChangeInnerRotation`
  (params (NewInner :type "Float (double-precision)"))
  (`self.SetRotationInner` (- (`self.ModuloAngle` NewInner) (`self.ModuloAngle` (`self.AccumulatedRotation`))))
  (`self.SetInnerTransform`)
  (`self.AppliedInnerMovement` (`self.RotationBase`)))

(fn `GetAccumulatedRotation`
  (returns (RotationAccumulated :type "Float (double-precision)"))
  (return (`self.AccumulatedRotation`)))

(fn `GetCurrentInnerRotation`
  (returns (InnerRotation :type "Float (double-precision)"))
  (if (`self.bIsInFailedRot`)
    (return (`self.InnerRotationAtStart`))
    (else
      (return (`self.InnerRotation`)))))

(fn `GetObjectTransform`
  (returns (Transform :type "Transform Structure"))
  (return (`SceneComponent.K2_GetComponentToWorld` (`self.RotationBase`))))

(fn `GetObjectTransformRelative`
  (returns (RelativeTransform :type "Transform Structure"))
  (return (`SceneComponent.GetRelativeTransform` (`self.RotationBase`))))

(fn `GetPlayerInRange`
  (params (PlayerPosition :type "Vector Structure"))
  (returns (PlayerInRange :type Boolean))
  (return (<= (`KismetMathLibrary.Vector_Distance2D` PlayerPosition (`SceneComponent.K2_GetComponentLocation` (`self.RotationBase`))) (`self.GetRange`))))

(fn `GetRange`
  (returns (Range :type "Float (double-precision)"))
  (bind _returnvalue_x (`KismetMathLibrary.BreakVector` (`SceneComponent.K2_GetComponentScale` (`self.RotationBase`))))
  (return (+ (* _returnvalue_x 50.0) 30.0)))

(fn `GetRotAngleToSave`
  (returns (AngleToSave :type "Float (double-precision)") (AccumulatedToSave :type "Float (double-precision)"))
  (bind _anglemodulo (`self.ModuloAngle` (`self.InnerRotationAtStart`)))
  (bind _anglemodulo_2 (`self.ModuloAngle` (+ (`self.InnerRotationAtStart`) (* (`CurveFloat.GetFloatValue` (`self.StandardRotationCurve`) (`self.StandardRotationEndTime`)) (`self.StandardRotationAngle`)))))
  (`self.CheckRotationState` "NewEnumerator1"
    (:`True`
      (if (< (/ (`self.StandardRotationTimer`) (`self.StandardRotationEndTime`)) 0.5)
        (return _anglemodulo (- (`self.AccumulatedRotation`) (- (`self.ModuloAngle` (`self.AccumulatedRotation`)) _anglemodulo)))
        (else
          (return _anglemodulo_2 (- (`self.AccumulatedRotation`) (- (`self.ModuloAngle` (`self.AccumulatedRotation`)) _anglemodulo_2))))))
    (:`False`
      (return (`self.InnerRotation`) (`self.AccumulatedRotation`)))))

(fn `GetRotationState`
  (returns (State :type "/Game/GPE/Moving/Rotation/E_RotationState Enum"))
  (return (`self.CurrentRotationState`)))

(fn `GetRotationSupportChilds`
  (returns (SupportsChilds :type "Array of /Game/GPE/Moving/Rotation/BP_RotationSupport Object Reference"))
  (bind _supportchildsfound (`self.RetrieveSupportChilds` self))
  (return _supportchildsfound))

(fn `GetRotSupportValues`
  (returns (Values :type "/Game/GPE/Moving/Rotation/PDA_RotSupportValues Object Reference"))
  (return (`self.SupportValues`)))

(fn `IsCurrentlyMoving`
  (returns (Moving :type Boolean))
  (return (`self.IsCurrentlyRotating`)))

(fn `IsCurrentlyRotating`
  (returns (Rotating :type Boolean))
  (switch `/Game/GPE/Moving/Rotation/E_RotationState` (`self.CurrentRotationState`)
    (:`NewEnumerator0`
      (return false))
    (:`NewEnumerator1`
      _)
    (:`NewEnumerator2`
      _)
    (:`NewEnumerator3`
      _))
  (return true))

(fn `LerpAngle`
  (params (A :type "Float (double-precision)") (B :type "Float (double-precision)") (Alpha :type "Float (double-precision)"))
  (returns (Return :type "Float (double-precision)"))
  (if (<= (`KismetMathLibrary.Abs` (- B A)) 180.0)
    (return (`KismetMathLibrary.Lerp` (`local.A`) (`local.B`) (`local.Alpha`)))
    (elif (< (`local.A`) (`local.B`))
      (return (`self.ModuloAngle` (`KismetMathLibrary.Lerp` (+ (`local.A`) 360.0) (`local.B`) (`local.Alpha`))))
      (else
        (return (`self.ModuloAngle` (`KismetMathLibrary.Lerp` (`local.A`) (+ (`local.B`) 360.0) (`local.Alpha`))))))))

(fn `RetrieveSupportChilds`
  (params (MovingObject :type "/Game/GPE/Moving/BP_MovingBase Object Reference"))
  (returns (SupportChildsFound :type "Array of /Game/GPE/Moving/Rotation/BP_RotationSupport Object Reference"))
  (locals (ReturnList :type "Array of /Game/GPE/Moving/Rotation/BP_RotationSupport Object Reference"))
  (for _array_element (`/Game/GPE/Moving/BP_MovingBase.MovableChilds` MovingObject)
    (bind _returnvalue (`ActorComponent.GetOwner` _array_element))
    (bind _asbp_rotation_support (cast `/Game/GPE/Moving/Rotation/BP_RotationSupport` _returnvalue)
      (:`then`
        (`KismetArrayLibrary.Array_AddUnique` (`local.ReturnList`) _asbp_rotation_support))
      (:`CastFailed`
        (bind _asbp_moving_base (cast `/Game/GPE/Moving/BP_MovingBase` _returnvalue))
        (bind _supportchildsfound (`self.RetrieveSupportChilds` _asbp_moving_base))
        (for _array_element_2 _supportchildsfound
          (`KismetArrayLibrary.Array_AddUnique` (`local.ReturnList`) _array_element_2)))))
  (return (`local.ReturnList`)))

(fn `SetInnerTransform`
  (bind _innertransform (`self.InnerTransform`))
  (set `self.InnerTransform` (`KismetMathLibrary.MakeTransform` (.location _innertransform) (`KismetMathLibrary.MakeRotator` (.roll (.rotation _innertransform)) (.pitch (.rotation _innertransform)) (- (`self.InnerRotation`) (.yaw (.rotation (`self.StartTransform`))))) (.scale _innertransform))))

(fn `SetOutlineVisibility`
  (params (Visibility :type Boolean))
  (`SceneComponent.SetVisibility` (`self.Outline`) Visibility false))

(fn `SetRotationInner`
  (params (InnerAdd :type "Float (double-precision)"))
  (bind _output_get (set `self.AccumulatedRotation` (+ InnerAdd (`self.AccumulatedRotation`))))
  (set `self.InnerRotation` (`self.ModuloAngle` _output_get)))

(fn `StartAutomaticRotation`
  (params (RotationSpeed :type "Float (double-precision)"))
  (set `self.CurrentRotationState` "NewEnumerator3")
  (set `self.AutomaticRotationSpeed` RotationSpeed)
  (set `self.bIsInFailedRot` false)
  (`self.StartMovementOnChildrens`))

(fn `StartControlledRotation`
  (params (RotationSpeed :type "Float (double-precision)") (RotStartupCurve :type "CurveFloat Object Reference") (RotStartupTime :type "Float (double-precision)"))
  (returns (RotationStarting :type Boolean))
  (switch `/Game/GPE/Moving/Rotation/E_RotationState` (`self.CurrentRotationState`)
    (:`NewEnumerator0`
      _)
    (:`NewEnumerator1`
      (return false))
    (:`NewEnumerator2`
      _)
    (:`NewEnumerator3`
      (return false))
    (:`NewEnumerator4`
      _))
  (set `self.CurrentRotationState` "NewEnumerator2")
  (set `self.ControlledRotSpeed` (`local.RotationSpeed`))
  (set `self.ControlledRotStartupCurve` (`local.RotStartupCurve`))
  (set `self.ControlledRotStartupTimer` 0.0)
  (set `self.ControlledRotStartupTime` (`local.RotStartupTime`))
  (`self.StartMovementOnChildrens`)
  (return true))

(fn `StartFailedRotation`
  (params (FailedRotationToLeft :type Boolean))
  (bind _supportvalues (`self.SupportValues`))
  (bind _failrotamplitude (`/Game/GPE/Moving/Rotation/PDA_RotSupportValues.FailRotAmplitude` (`self.SupportValues`)))
  (bind _rotationstarting (`self.StartStandardRotation` (`KismetMathLibrary.SelectFloat` (* -1.0 _failrotamplitude) _failrotamplitude FailedRotationToLeft) (`/Game/GPE/Moving/Rotation/PDA_RotSupportValues.FailRotDuration` _supportvalues) (`/Game/GPE/Moving/Rotation/PDA_RotSupportValues.FailRotCurve` _supportvalues)))
  (set `self.bIsInFailedRot` _rotationstarting))

(fn `StartStandardRotation`
  (params (RotationAngle :type "Float (double-precision)") (RotationDuration :type "Float (double-precision)") (RotationCurve :type "CurveFloat Object Reference"))
  (returns (RotationStarting :type Boolean))
  (`self.CheckRotationState` "NewEnumerator0"
    (:`True`
      (set `self.StandardRotationAngle` (`local.RotationAngle`))
      (set `self.StandardRotationCurve` (`local.RotationCurve`))
      (set `self.StandardRotationTimer` 0.0)
      (set `self.StandardRotationEndTime` (`local.RotationDuration`))
      (set `self.InnerRotationAtStart` (`self.AccumulatedRotation`))
      (set `self.CurrentRotationState` "NewEnumerator1")
      (`self.StartMovementOnChildrens`)
      (return true))
    (:`False`
      (return false))))

(fn `StopAutomaticRotation`
  (`self.CheckRotationState` "NewEnumerator3"
    (:`True`
      (set `self.CurrentRotationState` "NewEnumerator0")
      (set `self.bIsInFailedRot` false)
      (`self.StopMovementOnChildrens`))))

(fn `StopControlledRotation`
  (params (TriggerSnapping :type Boolean) (SnapAngle :type "Float (double-precision)") (FinishDuration :type "Float (double-precision)") (FinishCurve :type "CurveFloat Object Reference"))
  (switch `/Game/GPE/Moving/Rotation/E_RotationState` (`self.CurrentRotationState`)
    (:`NewEnumerator0`
      _)
    (:`NewEnumerator1`
      _)
    (:`NewEnumerator2`
      _)
    (:`NewEnumerator4`
      _))
  (if (`local.TriggerSnapping`)
    (set `self.CurrentRotationState` "NewEnumerator4")
    (set `self.ControlledRotFinishTimer` 0.0)
    (set `self.ControlledRotFinishTime` (`local.FinishDuration`))
    (set `self.ControlledRotFinishCurve` (`local.FinishCurve`))
    (set `self.ControlledRotSnapAngle` (`local.SnapAngle`))
    (set `self.InnerAtControlFinish` (`self.AccumulatedRotation`))
    (set `self.bIsInFailedRot` false)
    (`self.StartMovementOnChildrens`)
    (else
      (set `self.CurrentRotationState` "NewEnumerator0")
      (set `self.bIsInFailedRot` false)
      (`self.StopMovementOnChildrens`))))

(fn `UpdateClampVisual`
  (bind _clamplow (`self.ClampLow`))
  (bind _supportvalues (`self.SupportValues`))
  (bind _clamphigh (`self.ClampHigh`))
  (bind _relativescale3d_x (`KismetMathLibrary.BreakVector` (`SceneComponent.RelativeScale3D` (`self.RotationBase`))))
  (bind _relativescale3d_x_2 (`KismetMathLibrary.BreakVector` (`SceneComponent.RelativeScale3D` (`self.RotationBase`))))
  (`/Engine/EditorBlueprintResources/StandardMacros.IsValid` _supportvalues
    (:`Is Valid`
      (if (`/Game/GPE/Moving/Rotation/PDA_RotSupportValues.bUseClamp` _supportvalues)
        (`SceneComponent.SetVisibility` (`self.ClampLow`) true false)
        (`SceneComponent.SetVisibility` (`self.ClampHigh`) true false)
        (`|ExecutionSequence`
          (:`then_0`
            (`SceneComponent.SetWorldScale3D` (`self.ClampLow`) (* (`SceneComponent.K2_GetComponentScale` (`self.RotationBase`)) 0.5))
            (`SceneComponent.K2_SetRelativeRotation` _clamplow (`KismetMathLibrary.MakeRotator` 180.0 0.0 (`self.ModuloAngle` (+ (`/Game/GPE/Moving/Rotation/PDA_RotSupportValues.ClampLowValue` (`self.SupportValues`)) 180.0))) false false)
            (`SceneComponent.K2_SetRelativeLocation` _clamplow (`KismetMathLibrary.GreaterGreater_VectorRotator` (`KismetMathLibrary.MakeVector` (* _relativescale3d_x_2 -45.0) 0.0 -5.0) (`SceneComponent.K2_GetComponentRotation` (`self.ClampLow`))) false false))
          (:`then_1`
            (`SceneComponent.SetWorldScale3D` (`self.ClampHigh`) (* (`SceneComponent.K2_GetComponentScale` (`self.RotationBase`)) 0.5))
            (`SceneComponent.K2_SetRelativeRotation` _clamphigh (`KismetMathLibrary.MakeRotator` 180.0 0.0 (`self.ModuloAngle` (+ (`/Game/GPE/Moving/Rotation/PDA_RotSupportValues.ClampHighValue` (`self.SupportValues`)) 180.0))) false false)
            (`SceneComponent.K2_SetRelativeLocation` _clamphigh (`KismetMathLibrary.GreaterGreater_VectorRotator` (`KismetMathLibrary.MakeVector` (* _relativescale3d_x -45.0) 0.0 -5.0) (`SceneComponent.K2_GetComponentRotation` (`self.ClampHigh`))) false false)))
        (else
          (`SceneComponent.SetVisibility` (`self.ClampLow`) false false)
          (`SceneComponent.SetVisibility` (`self.ClampHigh`) false false))))))

(fn `UpdateControlledRotation`
  (params (NewControlledSpeed :type "Float (double-precision)"))
  (set `self.ControlledRotSpeed` NewControlledSpeed))

(fn `UserConstructionScript`
  (`self.UpdateClampVisual`))