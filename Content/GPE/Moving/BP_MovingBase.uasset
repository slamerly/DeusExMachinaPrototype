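; Base actor for moving gameplay objects that carry child BPAC_MovableObject components, with movement state and testing hooks left as stubs.
; Registered children are told to start moving, and to stop only once this actor and its own movable component are idle.
; Inner motion feeds that component when present, otherwise composes with the start transform.
; Editor helpers find children by MovingParent, recursing through nested moving objects to recompute offsets or apply test movement.
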(event `self.ReceiveBeginPlay`
  (bind _returnvalue (`self.GetComponentByClass` "/Game/GPE/Moving/BPAC_MovableObject.BPAC_MovableObject_C"))
  (`|ExecutionSequence`
    (:`then_0`
      (`/Engine/EditorBlueprintResources/StandardMacros.IsValid` _returnvalue
        (:`Is Valid`
          (set `self.bIsSelfMovable` true)
          (set `self.SelfMovable` _returnvalue))))
    (:`then_1`
      (set `self.StartTransform` (`self.GetTransform`)))))

(fn `AddMovable`
  (params (Movable :type "/Game/GPE/Moving/BPAC_MovableObject Object Reference"))
  (`KismetArrayLibrary.Array_AddUnique` (`self.MovableChilds`) Movable))

(fn `AppliedInnerMovement`
  (bind _innertransform (`self.InnerTransform`))
  (if (`self.bIsSelfMovable`)
    (set `/Game/GPE/Moving/BPAC_MovableObject.TransformMovingBase` _innertransform (`self.SelfMovable`))
    (else
      (`self.K2_SetActorTransform` (`KismetMathLibrary.ComposeTransforms` _innertransform (`self.StartTransform`))))))

(fn `ApplyChildsTestingEditor`
  (bind _childs (`self.RetrieveChildsEditor`))
  (for _array_element _childs
    (`|ExecutionSequence`
      (:`then_0`
        (`/Game/GPE/Moving/BPAC_MovableObject.ApplyTestingMovEditor` _array_element))
      (:`then_1`
        (bind (_ismovingobject _selfmovingobject) (`/Game/GPE/Moving/BPAC_MovableObject.IsSelfMovingObject` _array_element))
        (if _ismovingobject
          (`self.ApplyChildsTestingEditor` _selfmovingobject))))))

(fn `ApplyTestingValues`)

(fn `ComputeChildsOffsetEditor`
  (bind _childs (`self.RetrieveChildsEditor`))
  (for _array_element _childs
    (`|ExecutionSequence`
      (:`then_0`
        (bind (_ismovingobject _selfmovingobject) (`/Game/GPE/Moving/BPAC_MovableObject.IsSelfMovingObject` _array_element))
        (if _ismovingobject
          (`self.ComputeChildsOffsetEditor` _selfmovingobject)))
      (:`then_1`
        (`/Game/GPE/Moving/BPAC_MovableObject.RecomputeTransformOffset` _array_element)))))

(fn `GetObjectTransform`
  (returns (Transform :type "Transform Structure"))
  (return (`self.GetTransform`)))

(fn `IsCurrentlyMoving`
  (returns (Moving :type Boolean))
  (return false))

(fn `RetrieveChildsEditor`
  (returns (Childs :type "Array of /Game/GPE/Moving/BPAC_MovableObject Object Reference"))
  (locals (ReturnList :type "Array of /Game/GPE/Moving/BPAC_MovableObject Object Reference"))
  (bind _outactors (`LevelUtilitiesFunctions.GetAllActorsOfClassInLevel` (`self.GetLevel`) "/Script/Engine.Actor"))
  (for _array_element _outactors
    (bind _returnvalue (`self.GetComponentByClass` _array_element "/Game/GPE/Moving/BPAC_MovableObject.BPAC_MovableObject_C"))
    (`/Engine/EditorBlueprintResources/StandardMacros.IsValid` _returnvalue
      (:`Is Valid`
        (if (== (`/Game/GPE/Moving/BPAC_MovableObject.MovingParent` _returnvalue) self)
          (`KismetArrayLibrary.Array_AddUnique` (`local.ReturnList`) _returnvalue)))))
  (return (`local.ReturnList`)))

(fn `StartMovementOnChildrens`
  (for _array_element (`self.MovableChilds`)
    (`/Game/GPE/Moving/BPAC_MovableObject.SetMoving` _array_element true)))

(fn `StopMovementOnChildrens`
  (if (`self.IsCurrentlyMoving`)
    _
    (elif (`self.bIsSelfMovable`)
      (if (not (`/Game/GPE/Moving/BPAC_MovableObject.IsMoving` (`self.SelfMovable`)))
        (for _array_element (`self.MovableChilds`) :!label _label
          (`/Game/GPE/Moving/BPAC_MovableObject.SetMoving` _array_element false)))
      (else
        (goto _label)))))

(fn `UserConstructionScript`)