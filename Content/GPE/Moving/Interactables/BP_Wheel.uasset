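; Interactable wheel that the player grabs as a heavy interaction to drive linked rotation supports and moving platforms.
; Links lacking their controlled-rotation or A-to-B movement component are flagged at construction, and valid ones are cached at BeginPlay.
; Grab and release pass control to those components and swap materials.
; While held, stick X or optional circular-motion detection, with brief direction memory, spins the wheel and updates every linked component.
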(event `self.ReceiveBeginPlay`
  (`|ExecutionSequence`
    (:`then_0`
      (`self.ChangeMaterial` false))
    (:`then_1`
      ;[1 1 1] Check Linked Rot Supports
      (for _array_element (`self.LinkedRotSupports`)
        (bind (_rotationsupport _rotationvalues) (break `/Game/GPE/Moving/Interactables/STR_ControlledRotLink` _array_element))
        (`/Engine/EditorBlueprintResources/StandardMacros.IsValid` _rotationvalues
          (:`Is Valid`
            (`/Engine/EditorBlueprintResources/StandardMacros.IsValid` _rotationsupport
              (:`Is Valid`
                (bind _returnvalue (`self.GetComponentByClass` _rotationsupport "/Game/GPE/Moving/Rotation/BPAC_RotSupport_ControlledRotation.BPAC_RotSupport_ControlledRotation_C"))
                (`/Engine/EditorBlueprintResources/StandardMacros.IsValid` _returnvalue
                  (:`Is Valid`
                    (`KismetArrayLibrary.Array_Add` (`self.LinkedRotSupportsVerified`) (make `/Game/GPE/Moving/Interactables/STR_ControlledRotLink` _rotationsupport _rotationvalues _returnvalue))))))))))
    (:`then_2`
      ;[1 1 1] Check Linked Mov Platforms
      (for _array_element_2 (`self.LinkedMovPlatforms`)
        (bind (_movingplatform _movementvalues) (break `/Game/GPE/Moving/Interactables/STR_AToBMovLink` _array_element_2))
        (`/Engine/EditorBlueprintResources/StandardMacros.IsValid` _movementvalues
          (:`Is Valid`
            (`/Engine/EditorBlueprintResources/StandardMacros.IsValid` _movingplatform
              (:`Is Valid`
                (bind _returnvalue_2 (`self.GetComponentByClass` _movingplatform "/Game/GPE/Moving/MovingPlatforms/BPAC_MovPlatform_AToBMovement.BPAC_MovPlatform_AToBMovement_C"))
                (`/Engine/EditorBlueprintResources/StandardMacros.IsValid` _returnvalue_2
                  (:`Is Valid`
                    (`KismetArrayLibrary.Array_Add` (`self.LinkedMovPlatformsVerified`) (make `/Game/GPE/Moving/Interactables/STR_AToBMovLink` _movingplatform _movementvalues _returnvalue_2))))))))))))

(event `self.Interaction`
  (`self.ChangeMaterial` true)
  (set `self.bInInteraction` true)
  (`self.OnWheelGrab`)
  ;[1 1 1] Gain Control
  (`|ExecutionSequence`
    (:`then_0`
      (for _array_element (`self.LinkedRotSupportsVerified`)
        (bind (_rotationsupport _rotationvalues _controlledrotationcomponent) (break `/Game/GPE/Moving/Interactables/STR_ControlledRotLink` _array_element))
        (`/Game/GPE/Moving/Rotation/BPAC_RotSupport_ControlledRotation.GainControl` _controlledrotationcomponent _rotationvalues)))
    (:`then_1`
      (for _array_element_2 (`self.LinkedMovPlatformsVerified`)
        (bind (_movingplatform _movementvalues _abmovementcomponent) (break `/Game/GPE/Moving/Interactables/STR_AToBMovLink` _array_element_2))
        (`/Game/GPE/Moving/MovingPlatforms/BPAC_MovPlatform_AToBMovement.GainControl` _abmovementcomponent _movementvalues)))))

(event `self.InteractionHeavyFinished`
  (`self.ChangeMaterial` false)
  (set `self.bInInteraction` false)
  (`self.OnWheelReleased`)
  ;[1 1 1] Lose Control
  (`|ExecutionSequence`
    (:`then_0`
      (for _array_element (`self.LinkedRotSupportsVerified`)
        (`/Game/GPE/Moving/Rotation/BPAC_RotSupport_ControlledRotation.LoseControl` (`.ControlledRotationComponent_12_372D27E548F7515CB0E524AA22B57002` (break `/Game/GPE/Moving/Interactables/STR_ControlledRotLink` _array_element)))))
    (:`then_1`
      (for _array_element_2 (`self.LinkedMovPlatformsVerified`)
        (`/Game/GPE/Moving/MovingPlatforms/BPAC_MovPlatform_AToBMovement.LoseControl` (`.AbMovementComponent_6_8F29625E4DF549EEB892DA94C6D4CF13` (break `/Game/GPE/Moving/Interactables/STR_AToBMovLink` _array_element_2)))))))

(event `self.InteractionHeavyUpdate`
  (params (ControlValue :type "Vector2D Structure"))
  (bind _currentcontrolvalue (`self.CurrentControlValue`))
  (if (and (`self.bInInteraction`) (not (`self.IsControllerDisabled`)))
    (if (`self.bActivateJoystickCircles`)
      (bind _controlvalue (`self.ControlJoystickCircles` ControlValue))
      (set `self.CurrentControlValue` _controlvalue)
      (else
        (set `self.CurrentControlValue` (`KismetMathLibrary.BreakVector2D` ControlValue))))
    (`self.OnWheelUpdate` _currentcontrolvalue)
    (`|ExecutionSequence`
      (:`then_0`
        (`SceneComponent.K2_AddLocalRotation` (`self.Wheel`) (`KismetMathLibrary.MakeRotator` 0.0 0.0 (* (`self.CurrentControlValue`) (`GameplayStatics.GetWorldDeltaSeconds`) (`self.WheelVisualSpeed`))) false false))
      (:`then_1`
        ;[1 1 1] Update Control
        (for _array_element (`self.LinkedRotSupportsVerified`)
          (`/Game/GPE/Moving/Rotation/BPAC_RotSupport_ControlledRotation.UpdateControl` (`.ControlledRotationComponent_12_372D27E548F7515CB0E524AA22B57002` (break `/Game/GPE/Moving/Interactables/STR_ControlledRotLink` _array_element)) _currentcontrolvalue)))
      (:`then_2`
        (for _array_element_2 (`self.LinkedMovPlatformsVerified`)
          (`/Game/GPE/Moving/MovingPlatforms/BPAC_MovPlatform_AToBMovement.UpdateControl` (`.AbMovementComponent_6_8F29625E4DF549EEB892DA94C6D4CF13` (break `/Game/GPE/Moving/Interactables/STR_AToBMovLink` _array_element_2)) _currentcontrolvalue))))))

(fn `CanInteract`
  (returns (bIsInteractable :type Boolean))
  (return (not (`self.IsControllerDisabled`))))

(fn `ChangeMaterial`
  (params (Interact :type Boolean))
  (locals (Material :type "MaterialInterface Object Reference"))
  (set `local.Material` (select `bool` Interact :`false` (`self.MaterialNonInteract`) :`true` (`self.MaterialInteract`)))
  (`PrimitiveComponent.SetMaterial` (`self.Wheel`) 0 (`local.Material`))
  (`PrimitiveComponent.SetMaterial` (`self.Handle1`) 0 (`local.Material`))
  (`PrimitiveComponent.SetMaterial` (`self.Handle2`) 0 (`local.Material`))
  (`PrimitiveComponent.SetMaterial` (`self.Handle3`) 0 (`local.Material`))
  (`PrimitiveComponent.SetMaterial` (`self.Handle4`) 0 (`local.Material`))
  (`PrimitiveComponent.SetMaterial` (`self.Handle5`) 0 (`local.Material`))
  (`PrimitiveComponent.SetMaterial` (`self.Handle6`) 0 (`local.Material`))
  (`PrimitiveComponent.SetMaterial` (`self.Handle7`) 0 (`local.Material`))
  (`PrimitiveComponent.SetMaterial` (`self.Handle8`) 0 (`local.Material`)))

(fn `ControlJoystickCircles`
  (params (JoystickValue :type "Vector2D Structure"))
  (returns (ControlValue :type "Float (double-precision)"))
  (locals (NewJoystickAngle :type "Float (double-precision)") (Control :type "Float (double-precision)"))
  (bind _signeddelta (`self.SignedDeltaAngle` (`self.JoystickAngle`) (`local.NewJoystickAngle`)))
  (bind _returnvalue (`KismetMathLibrary.Abs` _signeddelta))
  (if (!= JoystickValue (0.0 0.0))
    (`|ExecutionSequence`
      (:`then_0`
        (set `local.NewJoystickAngle` (`KismetMathLibrary.DegAcos` (`KismetMathLibrary.DotProduct2D` (`local.JoystickValue`) (`KismetMathLibrary.MakeVector2D` 0.0 1.0))))
        (set `local.NewJoystickAngle` (`KismetMathLibrary.SelectFloat` (- 360.0 (`local.NewJoystickAngle`)) (`local.NewJoystickAngle`) (< (`KismetMathLibrary.BreakVector2D` (`local.JoystickValue`)) 0.0))))
      (:`then_1`
        (if (and (< _returnvalue 45.0) (> _returnvalue 5.0))
          (set `local.Control` (`KismetMathLibrary.SignOfFloat` _signeddelta))))
      (:`then_2`
        (set `self.JoystickAngle` (`local.NewJoystickAngle`))
        (if (!= (`local.Control`) 0.0)
          (set `self.JoystickLastControl` (`local.Control`))
          (set `self.JoystickForgotTime` (`KismetSystemLibrary.GetGameTimeInSeconds`))))
      (:`then_3`
        (if (!= (`local.Control`) 0.0)
          (return (`local.Control`))
          (elif (< (- (`KismetSystemLibrary.GetGameTimeInSeconds`) (`self.JoystickForgotTime`)) 0.2)
            (return (`self.JoystickLastControl`))
            (else
              (return 0.0))))))
    (else
      (return 0.0))))

(fn `ForceReleaseController`
  (`self.InteractionHeavyFinished`)
  (message `/Game/Player/BPI_PlayerController.SetPlayerInputMode` (`GameplayStatics.GetPlayerController` 0) "NewEnumerator0"))

(fn `IsHeavy`
  (returns (Heavy :type Boolean))
  (return true))

(fn `ModuloAngleBase360`
  (params (Angle :type "Float (double-precision)"))
  (returns (AngleModulo :type "Float (double-precision)"))
  (bind _returnvalue (mod Angle 360.0))
  (return (`KismetMathLibrary.SelectFloat` _returnvalue (+ _returnvalue 360.0) (>= _returnvalue 0.0))))

(fn `SignedDeltaAngle`
  (params (AngleFrom :type "Float (double-precision)") (AngleTo :type "Float (double-precision)"))
  (returns (SignedDelta :type "Float (double-precision)"))
  (bind _anglemodulo (`self.ModuloAngleBase360` (- (`self.ModuloAngleBase360` AngleTo) (`self.ModuloAngleBase360` AngleFrom))))
  (bind _returnvalue (- 360.0 _anglemodulo))
  (return (`KismetMathLibrary.SelectFloat` _anglemodulo (* _returnvalue -1.0) (< _anglemodulo _returnvalue))))

(fn `UserConstructionScript`
  (`|ExecutionSequence`
    (:`then_0`
      (for (_array_element _array_index) (`self.LinkedRotSupports`)
        (bind (_rotationsupport _rotationvalues) (break `/Game/GPE/Moving/Interactables/STR_ControlledRotLink` _array_element))
        (`/Engine/EditorBlueprintResources/StandardMacros.IsValid` _rotationsupport
          (:`Is Valid`
            (`/Engine/EditorBlueprintResources/StandardMacros.IsValid` (`self.GetComponentByClass` _rotationsupport "/Game/GPE/Moving/Rotation/BPAC_RotSupport_ControlledRotation.BPAC_RotSupport_ControlledRotation_C")
              (:`Is Not Valid`
                (`KismetSystemLibrary.PrintText` (`|FormatText` "Warning ! Rotation Support \"{name}\" doesn't have the Controlled Rotation component !" (`KismetSystemLibrary.GetDisplayName` _rotationsupport)) true true (struct :`R` 1.0 :`G` 0.105882 :`A` 1.0) 5.0)
                (`KismetArrayLibrary.Array_Set` (`self.LinkedRotSupports`) _array_index (make `/Game/GPE/Moving/Interactables/STR_ControlledRotLink` null _rotationvalues null))))))))
    (:`then_1`
      (for (_array_element_2 _array_index_2) (`self.LinkedMovPlatforms`)
        (bind (_movingplatform _movementvalues) (break `/Game/GPE/Moving/Interactables/STR_AToBMovLink` _array_element_2))
        (`/Engine/EditorBlueprintResources/StandardMacros.IsValid` _movingplatform
          (:`Is Valid`
            (`/Engine/EditorBlueprintResources/StandardMacros.IsValid` (`self.GetComponentByClass` _movingplatform "/Game/GPE/Moving/MovingPlatforms/BPAC_MovPlatform_AToBMovement.BPAC_MovPlatform_AToBMovement_C")
              (:`Is Not Valid`
                (`KismetSystemLibrary.PrintText` (`|FormatText` "Warning ! Moving Platform \"{name}\" doesn't have the A to B Movement component !" (`KismetSystemLibrary.GetDisplayName` _movingplatform)) true true (struct :`R` 1.0 :`G` 0.105882 :`A` 1.0) 5.0)
                (`KismetArrayLibrary.Array_Set` (`self.LinkedMovPlatforms`) _array_index_2 (make `/Game/GPE/Moving/Interactables/STR_AToBMovLink` null _movementvalues null))))))))))