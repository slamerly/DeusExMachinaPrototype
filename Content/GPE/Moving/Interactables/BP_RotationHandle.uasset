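; Heavy interactable handle that lets the player drive the controlled rotation of a linked rotation support.
; Construction sets that support as the movable component's parent, or warns and clears the link if it lacks BPAC_RotSupport_ControlledRotation; BeginPlay caches the component.
; Interaction swaps the handle material and gains or releases control.
; Updates send the dot product of axis-swapped input and ClockwiseArrow's 2D forward, giving a signed rotation input.
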(event `self.ReceiveBeginPlay`
  (bind (_rotationsupport _rotationvalues) (break `/Game/GPE/Moving/Interactables/STR_ControlledRotLink` (`self.LinkedSupport`)))
  (bind _returnvalue (`self.GetComponentByClass` _rotationsupport "/Game/GPE/Moving/Rotation/BPAC_RotSupport_ControlledRotation.BPAC_RotSupport_ControlledRotation_C"))
  (`|ExecutionSequence`
    (:`then_0`
      (`self.ChangeMaterial` false))
    (:`then_1`
      (`/Engine/EditorBlueprintResources/StandardMacros.IsValid` _rotationsupport
        (:`Is Valid`
          (`/Engine/EditorBlueprintResources/StandardMacros.IsValid` _returnvalue
            (:`Is Valid`
              (set `self.LinkedSupport` (make `/Game/GPE/Moving/Interactables/STR_ControlledRotLink` _rotationsupport _rotationvalues _returnvalue))
              (set `self.bLinkValid` true))))))))

(event `/Game/Interface/BPI_Interaction.Interaction`
  (bind (_rotationsupport _rotationvalues _standardrotationcomponent) (break `/Game/GPE/Moving/Interactables/STR_ControlledRotLink` (`self.LinkedSupport`)))
  (`self.ChangeMaterial` true)
  (set `self.bInInteraction` true)
  (`self.CheckLinkValid`
    (:`Valid`
      (`/Game/GPE/Moving/Rotation/BPAC_RotSupport_ControlledRotation.GainControl` _standardrotationcomponent _rotationvalues))))

(event `/Game/Interface/BPI_Interaction.InteractionHeavyFinished`
  (`self.ChangeMaterial` false)
  (set `self.bInInteraction` false)
  (`self.CheckLinkValid`
    (:`Valid`
      (`/Game/GPE/Moving/Rotation/BPAC_RotSupport_ControlledRotation.LoseControl` (`.StandardRotationComponent_11_372D27E548F7515CB0E524AA22B57002` (break `/Game/GPE/Moving/Interactables/STR_ControlledRotLink` (`self.LinkedSupport`)))))))

(event `/Game/Interface/BPI_Interaction.InteractionHeavyUpdate`
  (params (ControlValue :type "Vector2D Structure"))
  (bind (_x _y) (`KismetMathLibrary.BreakVector2D` ControlValue))
  (`self.CheckLinkValid`
    (:`Valid`
      (`/Game/GPE/Moving/Rotation/BPAC_RotSupport_ControlledRotation.UpdateControl` (`.StandardRotationComponent_11_372D27E548F7515CB0E524AA22B57002` (break `/Game/GPE/Moving/Interactables/STR_ControlledRotLink` (`self.LinkedSupport`))) (`KismetMathLibrary.DotProduct2D` (`KismetMathLibrary.MakeVector2D` _y _x) (`KismetMathLibrary.Conv_VectorToVector2D` (`SceneComponent.GetForwardVector` (`self.ClockwiseArrow`))))))))

(fn `CanInteract`
  (returns (bIsInteractable :type Boolean))
  (return true))

(fn `ChangeMaterial`
  (params (Interact :type Boolean))
  (locals (SelectedMaterial :type "MaterialInterface Object Reference"))
  (set `local.SelectedMaterial` (select `bool` Interact :`false` (`self.MaterialNonInteract`) :`true` (`self.MaterialInteract`)))
  (`PrimitiveComponent.SetMaterial` (`self.HandleVisual`) 0 (`local.SelectedMaterial`))
  (`PrimitiveComponent.SetMaterial` (`self.HandleVisual1`) 0 (`local.SelectedMaterial`)))

(fn `HideDefaultHandle`
  (`SceneComponent.SetVisibility` (`self.DefaultHandle`) false false)
  (`SceneComponent.SetVisibility` (`self.HandleVisual`) false false)
  (`SceneComponent.SetVisibility` (`self.HandleVisual1`) false false))

(fn `IsHeavy`
  (returns (Heavy :type Boolean))
  (return true))

(fn `ShowDefaultHandle`
  (`SceneComponent.SetVisibility` (`self.DefaultHandle`) true false)
  (`SceneComponent.SetVisibility` (`self.HandleVisual`) true false)
  (`SceneComponent.SetVisibility` (`self.HandleVisual1`) true false))

(fn `UserConstructionScript`
  (locals (AttemptSupport :type "/Game/GPE/Moving/Rotation/BP_RotationSupport Object Reference"))
  (bind (_rotationsupport _rotationvalues) (break `/Game/GPE/Moving/Interactables/STR_ControlledRotLink` (`self.LinkedSupport`)))
  (bind _output_get (set `local.AttemptSupport` _rotationsupport))
  (`/Engine/EditorBlueprintResources/StandardMacros.IsValid` _output_get
    (:`Is Valid`
      (`/Engine/EditorBlueprintResources/StandardMacros.IsValid` (`self.GetComponentByClass` (`local.AttemptSupport`) "/Game/GPE/Moving/Rotation/BPAC_RotSupport_ControlledRotation.BPAC_RotSupport_ControlledRotation_C")
        (:`Is Valid`
          (set `/Game/GPE/Moving/BPAC_MovableObject.MovingParent` (`local.AttemptSupport`) (`self.BPAC_MovableObject`)))
        (:`Is Not Valid`
          (`KismetSystemLibrary.PrintText` (`|FormatText` "Warning ! Rotation Support \"{name}\" doesn't have the Controlled Rotation component !" (`KismetSystemLibrary.GetDisplayName` (`local.AttemptSupport`))) true true (struct :`R` 1.0 :`G` 0.104343 :`A` 1.0) 5.0)
          (set `self.LinkedSupport` (make `/Game/GPE/Moving/Interactables/STR_ControlledRotLink` null _rotationvalues)))))))