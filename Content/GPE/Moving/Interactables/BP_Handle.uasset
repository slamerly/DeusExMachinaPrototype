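; Heavy interactable handle that lets the player drive a linked Rotation Support or Moving Platform, chosen by HandleControlMode.
; Construction script warns about and clears targets lacking the required control component, otherwise setting them as the handle's moving parent; BeginPlay caches that component.
; While held, it swaps material, fires grab/update/release callbacks and forwards stick input, projected onto ClockwiseArrow via 2D dot product, to the component.
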(event `self.ReceiveBeginPlay`
  (bind (_rotationsupport _rotationvalues) (break `/Game/GPE/Moving/Interactables/STR_ControlledRotLink` (`self.LinkedRotSupport`)))
  (bind (_movingplatform _movementvalues) (break `/Game/GPE/Moving/Interactables/STR_AToBMovLink` (`self.LinkedMovPlatform`)))
  (bind _returnvalue (`self.GetComponentByClass` _movingplatform "/Game/GPE/Moving/MovingPlatforms/BPAC_MovPlatform_AToBMovement.BPAC_MovPlatform_AToBMovement_C"))
  (bind _returnvalue_2 (`self.GetComponentByClass` _rotationsupport "/Game/GPE/Moving/Rotation/BPAC_RotSupport_ControlledRotation.BPAC_RotSupport_ControlledRotation_C"))
  (`|ExecutionSequence`
    (:`then_0`
      (`self.ChangeMaterial` false))
    (:`then_1`
      (switch `/Game/GPE/Moving/Interactables/E_HandleMode` (`self.HandleControlMode`)
        (:`NewEnumerator0`
          (`/Engine/EditorBlueprintResources/StandardMacros.IsValid` _rotationsupport
            (:`Is Valid`
              (`/Engine/EditorBlueprintResources/StandardMacros.IsValid` _returnvalue_2
                (:`Is Valid`
                  (set `self.LinkedRotSupport` (make `/Game/GPE/Moving/Interactables/STR_ControlledRotLink` _rotationsupport _rotationvalues _returnvalue_2))
                  (set `self.bLinkValid` true))))))
        (:`NewEnumerator1`
          (`/Engine/EditorBlueprintResources/StandardMacros.IsValid` _movingplatform
            (:`Is Valid`
              (`/Engine/EditorBlueprintResources/StandardMacros.IsValid` _returnvalue
                (:`Is Valid`
                  (set `self.LinkedMovPlatform` (make `/Game/GPE/Moving/Interactables/STR_AToBMovLink` _movingplatform _movementvalues _returnvalue))
                  (set `self.bLinkValid` true))))))))))

(event `/Game/Interface/BPI_Interaction.Interaction`
  (bind (_rotationsupport _rotationvalues _controlledrotationcomponent) (break `/Game/GPE/Moving/Interactables/STR_ControlledRotLink` (`self.LinkedRotSupport`)))
  (bind (_movingplatform _movementvalues _abmovementcomponent) (break `/Game/GPE/Moving/Interactables/STR_AToBMovLink` (`self.LinkedMovPlatform`)))
  (`self.ChangeMaterial` true)
  (set `self.bInInteraction` true)
  (`self.OnHandleGrab`)
  (`self.CheckLinkValid`
    (:`Valid`
      (switch `/Game/GPE/Moving/Interactables/E_HandleMode` (`self.HandleControlMode`)
        (:`NewEnumerator0`
          (`/Game/GPE/Moving/Rotation/BPAC_RotSupport_ControlledRotation.GainControl` _controlledrotationcomponent _rotationvalues))
        (:`NewEnumerator1`
          (`/Game/GPE/Moving/MovingPlatforms/BPAC_MovPlatform_AToBMovement.GainControl` _abmovementcomponent _movementvalues))))))

(event `/Game/Interface/BPI_Interaction.InteractionHeavyFinished`
  (`self.ChangeMaterial` false)
  (set `self.bInInteraction` false)
  (`self.OnHandleReleased`)
  (`self.CheckLinkValid`
    (:`Valid`
      (switch `/Game/GPE/Moving/Interactables/E_HandleMode` (`self.HandleControlMode`)
        (:`NewEnumerator0`
          (`/Game/GPE/Moving/Rotation/BPAC_RotSupport_ControlledRotation.LoseControl` (`.ControlledRotationComponent_12_372D27E548F7515CB0E524AA22B57002` (break `/Game/GPE/Moving/Interactables/STR_ControlledRotLink` (`self.LinkedRotSupport`)))))
        (:`NewEnumerator1`
          (`/Game/GPE/Moving/MovingPlatforms/BPAC_MovPlatform_AToBMovement.LoseControl` (`.AbMovementComponent_6_8F29625E4DF549EEB892DA94C6D4CF13` (break `/Game/GPE/Moving/Interactables/STR_AToBMovLink` (`self.LinkedMovPlatform`)))))))))

(event `/Game/Interface/BPI_Interaction.InteractionHeavyUpdate`
  (params (ControlValue :type "Vector2D Structure"))
  (bind (_x _y) (`KismetMathLibrary.BreakVector2D` ControlValue))
  (bind _returnvalue (`KismetMathLibrary.DotProduct2D` (`KismetMathLibrary.MakeVector2D` _y _x) (`KismetMathLibrary.Conv_VectorToVector2D` (`SceneComponent.GetForwardVector` (`self.ClockwiseArrow`)))))
  (if (and (`self.bInInteraction`) (not (`self.IsControllerDisabled`)))
    (`self.OnHandleUpdate` _returnvalue)
    (`self.CheckLinkValid`
      (:`Valid`
        (switch `/Game/GPE/Moving/Interactables/E_HandleMode` (`self.HandleControlMode`)
          (:`NewEnumerator0`
            (`/Game/GPE/Moving/Rotation/BPAC_RotSupport_ControlledRotation.UpdateControl` (`.ControlledRotationComponent_12_372D27E548F7515CB0E524AA22B57002` (break `/Game/GPE/Moving/Interactables/STR_ControlledRotLink` (`self.LinkedRotSupport`))) _returnvalue))
          (:`NewEnumerator1`
            (`/Game/GPE/Moving/MovingPlatforms/BPAC_MovPlatform_AToBMovement.UpdateControl` (`.AbMovementComponent_6_8F29625E4DF549EEB892DA94C6D4CF13` (break `/Game/GPE/Moving/Interactables/STR_AToBMovLink` (`self.LinkedMovPlatform`))) _returnvalue)))))))

(fn `CanInteract`
  (returns (bIsInteractable :type Boolean))
  (return (not (`self.IsControllerDisabled`))))

(fn `ChangeMaterial`
  (params (Interact :type Boolean))
  (locals (SelectedMaterial :type "MaterialInterface Object Reference"))
  (set `local.SelectedMaterial` (select `bool` Interact :`false` (`self.MaterialNonInteract`) :`true` (`self.MaterialInteract`)))
  (`PrimitiveComponent.SetMaterial` (`self.HandleVisual`) 0 (`local.SelectedMaterial`))
  (`PrimitiveComponent.SetMaterial` (`self.HandleVisual1`) 0 (`local.SelectedMaterial`)))

(fn `HideDefaultHandle`
  (`SceneComponent.SetVisibility` (`self.DefaultHandle`) false false)
  (`SceneComponent.SetVisibility` (`self.HandleVisual`) false false)
  (`SceneComponent.SetVisibility` (`self.HandleVisual1`) false false))

(fn `IsHeavy`
  (returns (Heavy :type Boolean))
  (return true))

(fn `ShowDefaultHandle`
  (`SceneComponent.SetVisibility` (`self.DefaultHandle`) true false)
  (`SceneComponent.SetVisibility` (`self.HandleVisual`) true false)
  (`SceneComponent.SetVisibility` (`self.HandleVisual1`) true false))

(fn `UserConstructionScript`
  (locals (AttemptSupport :type "/Game/GPE/Moving/Rotation/BP_RotationSupport Object Reference") (AttemptPlatform :type "/Game/GPE/Moving/MovingPlatforms/BP_MovingPlatform Object Reference"))
  (bind (_rotationsupport _rotationvalues) (break `/Game/GPE/Moving/Interactables/STR_ControlledRotLink` (`self.LinkedRotSupport`)))
  (bind (_movingplatform _movementvalues) (break `/Game/GPE/Moving/Interactables/STR_AToBMovLink` (`self.LinkedMovPlatform`)))
  (switch `/Game/GPE/Moving/Interactables/E_HandleMode` (`self.HandleControlMode`)
    (:`NewEnumerator0`
      (bind _output_get (set `local.AttemptSupport` _rotationsupport))
      (`/Engine/EditorBlueprintResources/StandardMacros.IsValid` _output_get
        (:`Is Valid`
          (`/Engine/EditorBlueprintResources/StandardMacros.IsValid` (`self.GetComponentByClass` (`local.AttemptSupport`) "/Game/GPE/Moving/Rotation/BPAC_RotSupport_ControlledRotation.BPAC_RotSupport_ControlledRotation_C")
            (:`Is Valid`
              (set `/Game/GPE/Moving/BPAC_MovableObject.MovingParent` (`local.AttemptSupport`) (`self.BPAC_MovableObject`)))
            (:`Is Not Valid`
              (`KismetSystemLibrary.PrintText` (`|FormatText` "Warning ! Rotation Support \"{name}\" doesn't have the Controlled Rotation component !" (`KismetSystemLibrary.GetDisplayName` (`local.AttemptSupport`))) true true (struct :`R` 1.0 :`G` 0.105882 :`A` 1.0) 5.0)
              (set `self.LinkedRotSupport` (make `/Game/GPE/Moving/Interactables/STR_ControlledRotLink` null _rotationvalues null)))))))
    (:`NewEnumerator1`
      (bind _output_get_2 (set `local.AttemptPlatform` _movingplatform))
      (`/Engine/EditorBlueprintResources/StandardMacros.IsValid` _output_get_2
        (:`Is Valid`
          (`/Engine/EditorBlueprintResources/StandardMacros.IsValid` (`self.GetComponentByClass` (`local.AttemptPlatform`) "/Game/GPE/Moving/MovingPlatforms/BPAC_MovPlatform_AToBMovement.BPAC_MovPlatform_AToBMovement_C")
            (:`Is Valid`
              (set `/Game/GPE/Moving/BPAC_MovableObject.MovingParent` (`local.AttemptPlatform`) (`self.BPAC_MovableObject`)))
            (:`Is Not Valid`
              (`KismetSystemLibrary.PrintText` (`|FormatText` "Warning ! Moving Platform \"{name}\" doesn't have the A To B Movement component !" (`KismetSystemLibrary.GetDisplayName` (`local.AttemptPlatform`))) true true (struct :`R` 1.0 :`G` 0.105882 :`A` 1.0) 5.0)
              (set `self.LinkedMovPlatform` (make `/Game/GPE/Moving/Interactables/STR_AToBMovLink` null _movementvalues null)))))))))