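; Interactable button that drives linked rotation supports and calls OnButtonPressed when used.
; The construction script warns about and clears linked supports lacking the matching standard or automatic rotation component, and BeginPlay caches the valid links.
; Interaction plays standard rotations and triggers automatic ones using each link's rotation values.
; A temporarily enabled Tick animates the press through a curve, blocking further interaction until it finishes.
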(event `self.ReceiveBeginPlay`
  (`|ExecutionSequence`
    (:`then_0`
      (set `self.ButtonBasePos` (`SceneComponent.K2_GetComponentLocation` (`self.Button`))))
    (:`then_1`
      ;[1 1 1] Check Linked Supports
      (for _array_element (`self.LinkedSupportsStandard`)
        (bind (_rotationsupport _rotationvalues) (break `/Game/GPE/Moving/Interactables/STR_StandardRotLink` _array_element))
        (`/Engine/EditorBlueprintResources/StandardMacros.IsValid` _rotationvalues
          (:`Is Valid`
            (`/Engine/EditorBlueprintResources/StandardMacros.IsValid` _rotationsupport
              (:`Is Valid`
                (bind _returnvalue (`self.GetComponentByClass` _rotationsupport "/Game/GPE/Moving/Rotation/BPAC_RotSupport_StandardRotation.BPAC_RotSupport_StandardRotation_C"))
                (`/Engine/EditorBlueprintResources/StandardMacros.IsValid` _returnvalue
                  (:`Is Valid`
                    (`KismetArrayLibrary.Array_Add` (`self.LinkedSupportsStdVerified`) (make `/Game/GPE/Moving/Interactables/STR_StandardRotLink` _rotationsupport _rotationvalues _returnvalue))))))))))
    (:`then_2`
      (for _array_element_2 (`self.LinkedSupportsAutomatic`)
        (bind (_rotationsupport_2 _rotationvalues_2) (break `/Game/GPE/Moving/Interactables/STR_AutomaticRotLink` _array_element_2))
        (`/Engine/EditorBlueprintResources/StandardMacros.IsValid` _rotationvalues_2
          (:`Is Valid`
            (`/Engine/EditorBlueprintResources/StandardMacros.IsValid` _rotationsupport_2
              (:`Is Valid`
                (bind _returnvalue_2 (`self.GetComponentByClass` _rotationsupport_2 "/Game/GPE/Moving/Rotation/BPAC_RotSupport_AutomaticRotation.BPAC_RotSupport_AutomaticRotation_C"))
                (`/Engine/EditorBlueprintResources/StandardMacros.IsValid` _returnvalue_2
                  (:`Is Valid`
                    (`KismetArrayLibrary.Array_Add` (`self.LinkedSupportsAutoVerified`) (make `/Game/GPE/Moving/Interactables/STR_AutomaticRotLink` _rotationsupport_2 _rotationvalues_2 _returnvalue_2))))))))))))

(event `self.ReceiveTick`
  (params (DeltaSeconds :type "Float (single-precision)"))
  ;[1 1 1] Visual Button Press
  (if (`self.bPressed`)
    (`|ExecutionSequence`
      (:`then_0`
        (bind _output_get (set `self.PressedTimer` (+ (`self.PressedTimer`) DeltaSeconds)))
        (if (>= _output_get (`self.PressedTime`))
          (set `self.PressedTimer` (`self.PressedTime`))
          (set `self.bPressed` false)
          (`self.SetActorTickEnabled` false)))
      (:`then_1`
        (`SceneComponent.K2_SetWorldLocation` (`self.Button`) (`KismetMathLibrary.VLerp` (`SceneComponent.K2_GetComponentLocation` (`self.ButtonPressedPos`)) (`self.ButtonBasePos`) (`CurveFloat.GetFloatValue` (`self.PressedCurve`) (/ (`self.PressedTimer`) (`self.PressedTime`)))) false false)))))

(event `/Game/Interface/BPI_Interaction.Interaction`
  (if (not (`self.bPressed`))
    (`|ExecutionSequence`
      (:`then_0`
        (set `self.bPressed` true)
        (set `self.PressedTimer` 0.0)
        (`self.SetActorTickEnabled` true))
      (:`then_1`
        (`self.OnButtonPressed`))
      (:`then_2`
        (for _array_element (`self.LinkedSupportsStdVerified`)
          (bind (_rotationsupport _rotationvalues _standardrotationcomponent) (break `/Game/GPE/Moving/Interactables/STR_StandardRotLink` _array_element))
          (`/Game/GPE/Moving/Rotation/BPAC_RotSupport_StandardRotation.PlayStandardRotation` _standardrotationcomponent _rotationvalues)))
      (:`then_3`
        (for _array_element_2 (`self.LinkedSupportsAutoVerified`)
          (bind (_rotationsupport_2 _rotationvalues_2 _automaticrotationcomponent) (break `/Game/GPE/Moving/Interactables/STR_AutomaticRotLink` _array_element_2))
          (`/Game/GPE/Moving/Rotation/BPAC_RotSupport_AutomaticRotation.TriggerAutoRotInteraction` _automaticrotationcomponent _rotationvalues_2))))))

(fn `CanInteract`
  (returns (bIsInteractable :type Boolean))
  (return (and (not (`self.bPressed`)) (not (`self.IsControllerDisabled`)))))

(fn `IsHeavy`
  (returns (Heavy :type Boolean))
  (return false))

(fn `UserConstructionScript`
  (`|ExecutionSequence`
    (:`then_0`
      (for (_array_element _array_index) (`self.LinkedSupportsStandard`)
        (bind (_rotationsupport _rotationvalues) (break `/Game/GPE/Moving/Interactables/STR_StandardRotLink` _array_element))
        (`/Engine/EditorBlueprintResources/StandardMacros.IsValid` _rotationsupport
          (:`Is Valid`
            (`/Engine/EditorBlueprintResources/StandardMacros.IsValid` (`self.GetComponentByClass` _rotationsupport "/Game/GPE/Moving/Rotation/BPAC_RotSupport_StandardRotation.BPAC_RotSupport_StandardRotation_C")
              (:`Is Not Valid`
                (`KismetSystemLibrary.PrintText` (`|FormatText` "Warning ! Rotation Support \"{name}\" doesn't have the Standard Rotation component !" (`KismetSystemLibrary.GetDisplayName` _rotationsupport)) true true (struct :`R` 1.0 :`G` 0.104343 :`A` 1.0) 5.0)
                (`KismetArrayLibrary.Array_Set` (`self.LinkedSupportsStandard`) _array_index (make `/Game/GPE/Moving/Interactables/STR_StandardRotLink` null _rotationvalues null))))))))
    (:`then_1`
      (for (_array_element_2 _array_index_2) (`self.LinkedSupportsAutomatic`)
        (bind (_rotationsupport_2 _rotationvalues_2) (break `/Game/GPE/Moving/Interactables/STR_AutomaticRotLink` _array_element_2))
        (`/Engine/EditorBlueprintResources/StandardMacros.IsValid` _rotationsupport_2
          (:`Is Valid`
            (`/Engine/EditorBlueprintResources/StandardMacros.IsValid` (`self.GetComponentByClass` _rotationsupport_2 "/Game/GPE/Moving/Rotation/BPAC_RotSupport_AutomaticRotation.BPAC_RotSupport_AutomaticRotation_C")
              (:`Is Not Valid`
                (`KismetSystemLibrary.PrintText` (`|FormatText` "Warning ! Rotation Support \"{name}\" doesn't have the Automatic Rotation component !" (`KismetSystemLibrary.GetDisplayName` _rotationsupport_2)) true true (struct :`R` 1.0 :`G` 0.104343 :`A` 1.0) 5.0)
                (`KismetArrayLibrary.Array_Set` (`self.LinkedSupportsAutomatic`) _array_index_2 (make `/Game/GPE/Moving/Interactables/STR_AutomaticRotLink` null _rotationvalues_2 null))))))))))