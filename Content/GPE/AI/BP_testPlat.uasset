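; BP_testPlat is a test platform that blocks AI navigation until it is raised.
; BeginPlay sets its nav modifier to the null area, and the `up` event switches it to the default area and plays a timeline.
; The timeline lerps the cube's current world Z toward Endpos on each update, keeping X and Y.
; The nodes that would capture Endpos and lower the cube beforehand are disconnected.
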(event `self.ReceiveBeginPlay`
  (`NavModifierComponent.SetAreaClass` (`self.NavModifier`) "/Script/NavigationSystem.NavArea_Null"))

(event `up`
  (bind (_returnvalue_x _returnvalue_y _returnvalue_z) (`KismetMathLibrary.BreakVector` (`SceneComponent.K2_GetComponentLocation` (`self.Cube`))))
  (`NavModifierComponent.SetAreaClass` (`self.NavModifier`) "/Script/NavigationSystem.NavArea_Default")
  (bind (_direction _newtrack_0) (`Timeline|Timeline`)
    (:`Update`
      (`SceneComponent.K2_SetWorldLocation` (`self.Cube`) (`KismetMathLibrary.MakeVector` _returnvalue_x _returnvalue_y (`KismetMathLibrary.Lerp` _returnvalue_z (`self.endpos`) _newtrack_0)) false false))))

(fn `UserConstructionScript`)