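; BP_LightStartingBackroom is a light that flickers on, apparently for the starting backroom area.
; BeginPlay and the SceneTransition event share one latent sequence that waits for Duration before switching the RectLight to NewIntensity.
; A chain of Delay nodes spaced by Blinkduration then toggles the intensity between zero and NewIntensity twice, leaving the light on.
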(event `self.ReceiveBeginPlay`
  (`KismetSystemLibrary.Delay` (`self.Duration`) :!label _label)
  (`LightComponent.SetIntensity` (`self.RectLight`) (`self.New Intensity`))
  (`KismetSystemLibrary.Delay` (`self.Blinkduration`))
  (`LightComponent.SetIntensity` (`self.RectLight`) 0.0)
  (`KismetSystemLibrary.Delay` (`self.Blinkduration`))
  (`LightComponent.SetIntensity` (`self.RectLight`) (`self.New Intensity`))
  (`KismetSystemLibrary.Delay` (`self.Blinkduration`))
  (`LightComponent.SetIntensity` (`self.RectLight`) 0.0)
  (`KismetSystemLibrary.Delay` (`self.Blinkduration`))
  (`LightComponent.SetIntensity` (`self.RectLight`) (`self.New Intensity`)))

(event `SceneTransition`
  (goto _label))

(fn `UserConstructionScript`)