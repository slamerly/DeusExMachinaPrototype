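; Trigger-box actor that blends the first local player's camera view to a player pawn when something overlaps it.
; The overlap tests for BPPC_Player, then BPC_Player_CameraTest, and both routes target the CameraTest cast result in a timed SetViewTargetWithBlend.
; Only the second route assigns that result, so the first has no fresh target.
; A fade-to-black widget sequence is present but disconnected and never runs.
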(event `self.Box.OnComponentBeginOverlap`
  (params (OverlappedComponent :type "PrimitiveComponent Object Reference") (OtherActor :type "Actor Object Reference") (OtherComp :type "PrimitiveComponent Object Reference") (OtherBodyIndex :type Integer) (bFromSweep :type Boolean) (SweepResult :type "HitResult Structure (by ref)"))
  (cast `/Game/Player/BPPC_Player` OtherActor
    (:`then`
      _)
    (:`CastFailed`
      (bind _asbpc_player_camera_test (cast `/Game/Player/BPC_Player_CameraTest` OtherActor))))
  (`PlayerController.SetViewTargetWithBlend` (`GameplayStatics.GetPlayerController` 0) _asbpc_player_camera_test 1.5 "VTBlend_Linear" 0.0 false))

(fn `UserConstructionScript`)