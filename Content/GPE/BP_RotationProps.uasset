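; BP_RotationProps is an interactable gameplay prop, named for rotation, whose interaction is a placeholder that only prints a debug string.
; The Interaction event calls CanInteract before printing.
; CanInteract returns the BPACInteractable component's Interactable flag when its sphere collision is enabled and otherwise allows interaction.
; No rotation logic is implemented in these graphs.
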(event `self.Interaction`
  (bind _bisinteractable (`self.CanInteract`))
  (if _bisinteractable
    (`KismetSystemLibrary.PrintString` "ca tourne")))

(fn `CanInteract`
  (returns (bIsInteractable :type Boolean))
  (bind _bpac_interactable (`self.BPAC_Interactable`))
  (if (`/Game/GPE/BPAC_Interactable.bEnableSphereCollision` _bpac_interactable)
    (`/Engine/EditorBlueprintResources/StandardMacros.IsValid` _bpac_interactable
      (:`Is Valid`
        (return (`/Game/GPE/BPAC_Interactable.bInteractable` _bpac_interactable))))
    (else
      (return true))))

(fn `UserConstructionScript`)