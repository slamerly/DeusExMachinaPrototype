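; In-scene door teleporter that moves the player pawn to a linked Destination teleporter.
; Overlapping the Box blocks player inputs, then a timeline lerps the pawn to the Back point and turns it to face into the door.
; After TravelTime, the pawn jumps to the Destination's Back, whose exit timeline slides it out to the actor's location and unblocks inputs.
; The Destination's Teleporting flag prevents retriggering on arrival, and a missing Destination prints an error.
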(event `self.ReceiveBeginPlay`
  (bind _asbppc_player (cast `/Game/Player/BPPC_Player` (`GameplayStatics.GetPlayerController` 0)))
  (set `self.PlayerController` _asbppc_player))

(event `AnimationEnterDoor`
  (bind (_playerposition_x _playerposition_y _playerposition_z) (`KismetMathLibrary.BreakVector` (`self.PlayerPosition`)))
  (bind (_returnvalue_x _returnvalue_y) (`KismetMathLibrary.BreakVector` (`SceneComponent.K2_GetComponentLocation` (`self.Back`))))
  ;[1 1 1] Animation Enter
  (bind (_direction _newtrack_0) (`Timeline|T_AnimationEnter` :!via `PlayFromStart`)
    (:`Update`
      (`self.K2_SetActorLocationAndRotation` (`GameplayStatics.GetPlayerPawn` 0) (`KismetMathLibrary.VLerp` (`KismetMathLibrary.MakeVector` _playerposition_x _playerposition_y _playerposition_z) (`KismetMathLibrary.MakeVector` _returnvalue_x _returnvalue_y _playerposition_z) _newtrack_0) (`KismetMathLibrary.RLerp` (`self.PlayerRotation`) (`KismetMathLibrary.Conv_VectorToRotator` (* (`self.GetActorRightVector`) -1.0)) _newtrack_0 true) false false))
    (:`Finished`
      (`self.Teleportation`))))

(event `Teleportation`
  (bind _destination (`self.Destination`))
  ;[0 1 1 0.33] Teleportation
  (`/Engine/EditorBlueprintResources/StandardMacros.IsValid` _destination
    (:`Is Valid`
      (set `/Game/GPE/BP_TeleportInsideScene.Teleporting` true _destination)
      (`KismetSystemLibrary.Delay` (`self.TravelTime`))
      (`self.K2_SetActorLocationAndRotation` (`GameplayStatics.GetPlayerPawn` 0) (`SceneComponent.K2_GetComponentLocation` (`/Game/GPE/BP_TeleportInsideScene.Back` _destination)) (`KismetMathLibrary.Conv_VectorToRotator` (`self.GetActorRightVector` _destination)) false true)
      (`self.AnimationExitDoor` (`self.Destination`)))
    (:`Is Not Valid`
      ;;[1 0 0 0.33] Error
      (`KismetSystemLibrary.PrintText` (`|FormatText` "Error: No destination for {this}" (`KismetSystemLibrary.GetObjectName` self)) true true (struct :`R` 1.0 :`A` 1.0) 12000.0))))

(event `AnimationExitDoor`
  (bind (_returnvalue_x _returnvalue_y) (`KismetMathLibrary.BreakVector` (`self.K2_GetActorLocation`)))
  (bind (_returnvalue_x_2 _returnvalue_y_2 _returnvalue_z) (`KismetMathLibrary.BreakVector` (`SceneComponent.K2_GetComponentLocation` (`self.Back`))))
  (bind _returnvalue (- _returnvalue_z 14.0))
  ;[1 1 1] Animation Exit
  (bind (_direction _newtrack_0) (`Timeline|T_AnimationExit` :!via `PlayFromStart`)
    (:`Update`
      (`self.K2_SetActorLocation` (`GameplayStatics.GetPlayerPawn` 0) (`KismetMathLibrary.VLerp` (`KismetMathLibrary.MakeVector` _returnvalue_x_2 _returnvalue_y_2 _returnvalue) (`KismetMathLibrary.MakeVector` _returnvalue_x _returnvalue_y _returnvalue) _newtrack_0) false false))
    (:`Finished`
      (`/Game/Player/BPPC_Player.UnblockPlayerInputs` (`self.PlayerController`) "NewEnumerator1")
      (set `self.Teleporting` false))))

(event `self.Box.OnComponentBeginOverlap`
  (params (OverlappedComponent :type "PrimitiveComponent Object Reference") (OtherActor :type "Actor Object Reference") (OtherComp :type "PrimitiveComponent Object Reference") (OtherBodyIndex :type Integer) (bFromSweep :type Boolean) (SweepResult :type "HitResult Structure (by ref)"))
  (bind _returnvalue (`GameplayStatics.GetPlayerPawn` 0))
  ;[1 1 1] Detection
  (if (and (== OtherActor (`GameplayStatics.GetPlayerPawn` 0)) (not (`self.Teleporting`)))
    (`/Game/Player/BPPC_Player.BlockPlayerInputs` (`self.PlayerController`) "NewEnumerator1")
    (set `self.PlayerPosition` (`self.K2_GetActorLocation` _returnvalue))
    (set `self.PlayerRotation` (`self.K2_GetActorRotation` _returnvalue))
    (`self.AnimationEnterDoor`)))

(fn `UserConstructionScript`)