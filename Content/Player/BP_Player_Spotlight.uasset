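; BP_Player_Spotlight is an actor whose spotlight tracks the player character.
; On BeginPlay it caches player character 0.
; Each Tick, while that reference is valid, it computes a look-at rotation toward the player's root component and turns the SpotLight toward it at a constant rate using RInterpToConstant.
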(event `self.ReceiveBeginPlay`
  (set `self.Player` (`GameplayStatics.GetPlayerCharacter` 0)))

(event `self.ReceiveTick`
  (params (DeltaSeconds :type "Float (single-precision)"))
  (bind _spotlight (`self.SpotLight`))
  (bind _player (`self.Player`))
  (`/Engine/EditorBlueprintResources/StandardMacros.IsValid` _player
    (:`Is Valid`
      (`SceneComponent.K2_SetWorldRotation` _spotlight (`KismetMathLibrary.RInterpTo_Constant` (`SceneComponent.K2_GetComponentRotation` _spotlight) (`KismetMathLibrary.FindLookAtRotation` (`SceneComponent.K2_GetComponentLocation` (`self.SpotLight`)) (`SceneComponent.K2_GetComponentLocation` (`Actor.RootComponent` _player))) (`GameplayStatics.GetWorldDeltaSeconds`) 100.0) false false))))

(fn `UserConstructionScript`)