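; Player character blueprint that switches the first player controller's view to a camera and detects interactable objects in front of the player.
; Each tick, a forward line trace stores any BPI_Interaction hit, toggles a prompt widget and outlines tagged meshes through custom depth stencil.
; The miss branch also leaves custom depth on, and the capsule overlap detection is disconnected.
; Helper functions toggle capsule collision on a custom channel and test whether an actor is ahead.
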(event `self.ReceiveBeginPlay`
  (`PlayerController.SetViewTargetWithBlend` (`GameplayStatics.GetPlayerController` 0) (`self.Camera`) 0.0 "VTBlend_Linear" 0.0 false))

(event `self.ReceiveTick`
  (params (DeltaSeconds :type "Float (single-precision)"))
  (bind _widget (`self.Widget`))
  (bind _returnvalue (- (`self.K2_GetActorLocation`) (0.0 0.0 50.0)))
  ;[1 1 1] Interaction Raycast
  (bind _outhit (`KismetSystemLibrary.LineTraceSingle` _returnvalue (+ _returnvalue (* (`self.GetActorForwardVector`) (`self.DistanceInteractionForw`))) "TraceTypeQuery1"))
  (bind (_bblockinghit _binitialoverlap _time _distance _location _impactpoint _normal _impactnormal _physmat _hitactor) (`GameplayStatics.BreakHitResult` _outhit))
  (if (`KismetSystemLibrary.DoesImplementInterface` _hitactor "/Game/Interface/BPI_Interaction.BPI_Interaction_C")
    (bind _output_get (set `self.ActorInteracted` _hitactor))
    (`self.Find Outline Meshes` _output_get)
    (`self.Set Outline Meshes Render Custom Depth` true)
    (`SceneComponent.SetVisibility` _widget true false)
    (else
      (set `self.ActorInteracted` null)
      (`self.Set Outline Meshes Render Custom Depth` true)
      (`SceneComponent.SetVisibility` _widget false false))))

(event `self.CapsuleComponent.OnComponentBeginOverlap`
  (params (OverlappedComponent :type "PrimitiveComponent Object Reference") (OtherActor :type "Actor Object Reference") (OtherComp :type "PrimitiveComponent Object Reference") (OtherBodyIndex :type Integer) (bFromSweep :type Boolean) (SweepResult :type "HitResult Structure (by ref)"))
  ;[1 1 1] Interaction with area
)

(event `self.CapsuleComponent.OnComponentEndOverlap`
  (params (OverlappedComponent :type "PrimitiveComponent Object Reference") (OtherActor :type "Actor Object Reference") (OtherComp :type "PrimitiveComponent Object Reference") (OtherBodyIndex :type Integer))
  ;[1 1 1] Interaction with area
)

(fn `Find Outline Meshes`
  (params (actor :type "Actor Object Reference"))
  (bind _outline_meshes (`self.Outline Meshes`))
  (`KismetArrayLibrary.Array_Clear` _outline_meshes)
  (for _array_element (`self.GetComponentsByTag` actor "/Script/Engine.MeshComponent" "Interaction Outline")
    (`PrimitiveComponent.SetCustomDepthStencilValue` _array_element 1)
    (`KismetArrayLibrary.Array_Add` _outline_meshes _array_element)))

(fn `IsInteracActorAreaForward`
  (params (InteractableActor :type "Actor Object Reference"))
  (returns (IsForward :type Boolean))
  (bind _returnvalue (- (`self.K2_GetActorLocation`) (0.0 0.0 50.0)))
  (bind _outhit (`KismetSystemLibrary.LineTraceSingle` _returnvalue (+ _returnvalue (* (`self.GetActorForwardVector`) (`self.DistanceInteractionForw`))) "TraceTypeQuery1"))
  (return (== (`.HitActor` (`GameplayStatics.BreakHitResult` _outhit)) InteractableActor)))

(fn `Set Outline Meshes Render Custom Depth`
  (params (`Is Visible` :type Boolean))
  (for _array_element (`self.Outline Meshes`)
    (`PrimitiveComponent.SetRenderCustomDepth` _array_element `Is Visible`)))

(fn `SetNoCollisionMode`
  (params (NoCollisionActivated :type Boolean))
  (bind _capsulecomponent (`self.CapsuleComponent`))
  (if NoCollisionActivated
    (`PrimitiveComponent.SetCollisionResponseToChannel` _capsulecomponent "ECC_GameTraceChannel1" "ECR_Ignore")
    (else
      (`PrimitiveComponent.SetCollisionResponseToChannel` _capsulecomponent "ECC_GameTraceChannel1" "ECR_Block"))))

(fn `UserConstructionScript`)