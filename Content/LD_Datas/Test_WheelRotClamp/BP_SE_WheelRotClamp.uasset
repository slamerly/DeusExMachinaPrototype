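; Test Blueprint that stops wheel interaction once a rotation support reaches its upper clamp limit.
; On BeginPlay it binds to the RotationSupport's clamp event.
; When the reported clamp angle equals the support's high clamp value, it disables the controller on the RotationWheel.
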(event `self.ReceiveBeginPlay`
  (bind _rotationsupport (`self.RotationSupport`))
  (`/Engine/EditorBlueprintResources/StandardMacros.IsValid` _rotationsupport
    (:`Is Valid`
      (add `/Game/GPE/Moving/Rotation/BP_RotationSupport.OnRotSupportClamp` _rotationsupport (delegate `On Clamp`)))))

(event `On Clamp`
  (params (ClampAngle :type "Float (double-precision)"))
  (bind _rotationwheel (`self.RotationWheel`))
  (if (== ClampAngle (`/Game/GPE/Moving/Rotation/PDA_RotSupportValues.ClampHighValue` (`/Game/GPE/Moving/Rotation/BP_RotationSupport.GetRotSupportValues` (`self.RotationSupport`))))
    (`/Engine/EditorBlueprintResources/StandardMacros.IsValid` _rotationwheel
      (:`Is Valid`
        (`/Game/GPE/Moving/Interactables/BP_InteractableBase.DisableController` _rotationwheel)))))

(fn `UserConstructionScript`)