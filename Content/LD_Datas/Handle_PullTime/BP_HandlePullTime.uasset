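; BP_HandlePullTime is a timed pull interaction that starts a Curtain sequence once a linked Handle has been pulled for long enough.
; It binds to the Handle's grab, release and update events, ticking only while held and resetting the timer on each grab.
; Tick fills the timer while the control value is below a threshold and drains it otherwise.
; Success locks out further pulls and force-releases the controller.
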(event `self.ReceiveBeginPlay`
  (bind _handle (`self.Handle`))
  (`/Engine/EditorBlueprintResources/StandardMacros.IsValid` _handle
    (:`Is Valid`
      (add `/Game/GPE/Moving/Interactables/BP_Handle.OnHandleGrab` _handle (delegate `HandleGrab`))
      (add `/Game/GPE/Moving/Interactables/BP_Handle.OnHandleReleased` _handle (delegate `HandleRelease`))
      (add `/Game/GPE/Moving/Interactables/BP_Handle.OnHandleUpdate` _handle (delegate `Handle Update`)))))

(event `HandleGrab`
  (`self.HandleGrabFunc`))

(event `HandleRelease`
  (`self.HandleReleaseFunc`))

(event `Handle Update`
  (params (ControlValue :type "Float (double-precision)"))
  (`self.HandleUpdateFunc` ControlValue))

(event `self.ReceiveTick`
  (params (DeltaSeconds :type "Float (single-precision)"))
  (`|ExecutionSequence`
    (:`then_0`
      (if (`self.bPullThisFrame`)
        (bind _output_get (set `self.Timer` (+ (`self.Timer`) DeltaSeconds)))
        (if (>= _output_get (`self.PullTimeNeeded`))
          (`self.PullSuccess`)
          (`/Game/GPE/Curtain_Juliette/BP_CurtainJuliet.StartSequence` (`self.Curtain`)))
        (else
          (set `self.Timer` (`KismetMathLibrary.FMax` (- (`self.Timer`) DeltaSeconds))))))
    (:`then_1`
      (if (`self.bPrintPullTimer`)
        (`KismetSystemLibrary.PrintString` (`KismetStringLibrary.Conv_DoubleToString` (`self.Timer`)) true true (struct :`R` 0.880731 :`G` 1.0 :`B` 0.479167 :`A` 1.0) 0.0)))))

(fn `HandleGrabFunc`
  (if (not (`self.bSuccess`))
    (set `self.Timer` 0.0)
    (`self.SetActorTickEnabled` true)))

(fn `HandleReleaseFunc`
  (`self.SetActorTickEnabled` false))

(fn `HandleUpdateFunc`
  (params (ControlValue :type "Float (double-precision)"))
  (if (not (`self.bSuccess`))
    (set `self.bPullThisFrame` (< ControlValue -0.5))))

(fn `PullSuccess`
  (set `self.bSuccess` true)
  (`self.SetActorTickEnabled` false)
  (`/Game/GPE/Moving/Interactables/BP_InteractableBase.ForceReleaseController` (`self.Handle`))
  (`KismetSystemLibrary.PrintString` "Pull Success!" true true (struct :`R` 0.063532 :`G` 1.0 :`A` 1.0) 5.0))

(fn `UserConstructionScript`)