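; BP_HUD_DeusEx is a HUD Blueprint that creates the game's debug and pause menu widgets.
; On BeginPlay it creates WBP_Debug and WBP_PauseMenu for player controller 0 and adds both to the viewport, with the debug widget layered above the pause menu.
; It stores both widget references and exposes them through GetDebugWidget and GetPauseWidget.
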(event `self.ReceiveBeginPlay`
  (bind _returnvalue (`GameplayStatics.GetPlayerController` 0))
  (`|ExecutionSequence`
    (:`then_0`
      (bind _returnvalue_2 (`|CreateWidget` "/Game/Debug/WBP_Debug.WBP_Debug_C" _returnvalue))
      (bind _output_get (set `self.DebugWidget` _returnvalue_2))
      (`UserWidget.AddToViewport` _output_get 1))
    (:`then_1`
      (bind _returnvalue_3 (`|CreateWidget` "/Game/Widget/Pause/WBP_PauseMenu.WBP_PauseMenu_C" _returnvalue))
      (bind _output_get_2 (set `self.PauseWidget` _returnvalue_3))
      (`UserWidget.AddToViewport` _output_get_2 0))))

(fn `GetDebugWidget`
  (returns (DebugWidget :type "/Game/Debug/WBP_Debug Object Reference"))
  (return (`self.DebugWidget`)))

(fn `GetPauseWidget`
  (returns (PauseWidget :type "/Game/Widget/Pause/WBP_PauseMenu Object Reference"))
  (return (`self.PauseWidget`)))

(fn `UserConstructionScript`)