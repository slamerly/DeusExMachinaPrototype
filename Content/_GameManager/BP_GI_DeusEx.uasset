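; Game instance that coordinates global save and load and keeps a map of save-game objects by slot name.
; Slot linking loads or creates each save object, while saving and loading message the BPI_Saver component on actors tagged "SaveGame".
; Loading blocks move input and restores the SceneManager first, then the rest after a short delay, to avoid a player problem.
; Init only prints DT_Timeline row names and fetches the "Initial" row without using it.
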(event `GlobalSave`
  (bind _outactors (`GameplayStatics.GetAllActorsWithTag` "SaveGame"))
  (for _array_element _outactors
    (message `/Game/Save/BPI_Saver.Save` (`|GetArrayItem` (`Actor.GetComponentsByInterface` _array_element "/Game/Save/BPI_Saver.BPI_Saver_C"))))
  (`KismetSystemLibrary.PrintString` "SaveGame" true true (struct :`R` 1.0 :`G` 1.0 :`A` 1.0) 3.0))

(event `GlobalLoad`
  (`Controller.SetIgnoreMoveInput` (`GameplayStatics.GetPlayerController` 0) true)
  ;[1 1 1] Load SceneManager before for dodge player problem
  (bind _returnvalue (`GameplayStatics.GetActorOfClass` (`|ConvertAsset` (`self.SoftClassSceneManager`))))
  (message `/Game/Save/BPI_Saver.Load` (`|GetArrayItem` (`Actor.GetComponentsByInterface` _returnvalue "/Game/Save/BPI_Saver.BPI_Saver_C")))
  (`KismetSystemLibrary.Delay` 0.1)
  (bind _outactors (`GameplayStatics.GetAllActorsWithTag` "SaveGame"))
  (for _array_element _outactors
    (if (!= _array_element _returnvalue)
      (message `/Game/Save/BPI_Saver.Load` (`|GetArrayItem` (`Actor.GetComponentsByInterface` _array_element "/Game/Save/BPI_Saver.BPI_Saver_C")))))
  (`Controller.SetIgnoreMoveInput` (`GameplayStatics.GetPlayerController` 0) false)
  (`KismetSystemLibrary.PrintString` "LoadGame" true true (struct :`R` 1.0 :`G` 1.0 :`A` 1.0) 3.0))

(event `self.ReceiveInit`
  (bind _outrownames (`DataTableFunctionLibrary.GetDataTableRowNames` "/Game/Save/Timeline/DT_Timeline.DT_Timeline"))
  (for _array_element _outrownames
    (`KismetSystemLibrary.PrintString` (`KismetStringLibrary.Conv_NameToString` _array_element)))
  (`|GetDataTableRow` "/Game/Save/Timeline/DT_Timeline.DT_Timeline" "Initial"))

(event `/Game/Interface/BPI_GameInstance.LinkSaveGameSlot`
  (params (SlotName :type String) (ClassSaveGame :type "SaveGame Class Reference"))
  (if (not (`BlueprintMapLibrary.Map_Contains` (`self.RefSaveSlot`) SlotName))
    (bind _returnvalue (`GameplayStatics.DoesSaveGameExist` SlotName))
    (if _returnvalue
      (bind _returnvalue_2 (`GameplayStatics.LoadGameFromSlot` SlotName))
      (`BlueprintMapLibrary.Map_Add` (`self.RefSaveSlot`) SlotName _returnvalue_2)
      (elif (`KismetSystemLibrary.IsValidClass` ClassSaveGame)
        (bind _returnvalue_3 (`GameplayStatics.CreateSaveGameObject` ClassSaveGame))
        (`BlueprintMapLibrary.Map_Add` (`self.RefSaveSlot`) SlotName _returnvalue_3)))))

(fn `GetSaveGameRef`
  (params (SlotName :type String))
  (returns (SaveGameRef :type "SaveGame Object Reference"))
  (bind (_value _returnvalue) (`BlueprintMapLibrary.Map_Find` (`self.RefSaveSlot`) SlotName))
  (if _returnvalue
    (return _value)
    (else
      (`KismetSystemLibrary.PrintString` "SlotName not found" true true (struct :`R` 1.0 :`A` 1.0)))))