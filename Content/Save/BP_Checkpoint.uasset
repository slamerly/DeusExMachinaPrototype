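; BP_Checkpoint is a trigger actor that records the player's transform as a checkpoint.
; On BeginPlay it finds and caches the BP_SceneManager in the level.
; When the player pawn overlaps its box, it passes the pawn's transform, raised slightly in Z, to the scene manager through CheckpointPlayerTransformMessage and prints that location for debugging.
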(event `self.ReceiveBeginPlay`
  (bind _returnvalue (`GameplayStatics.GetActorOfClass` "/Game/SceneManagement/BP_SceneManager.BP_SceneManager_C"))
  (set `self.SceneManager` _returnvalue))

(event `self.Box.OnComponentBeginOverlap`
  (params (OverlappedComponent :type "PrimitiveComponent Object Reference") (OtherActor :type "Actor Object Reference") (OtherComp :type "PrimitiveComponent Object Reference") (OtherBodyIndex :type Integer) (bFromSweep :type Boolean) (SweepResult :type "HitResult Structure (by ref)"))
  (bind _returnvalue (`GameplayStatics.GetPlayerPawn` 0))
  (bind (_returnvalue_location _returnvalue_rotation _returnvalue_scale) (`KismetMathLibrary.BreakTransform` (`self.GetTransform` _returnvalue)))
  (bind _returnvalue_2 (+ _returnvalue_location (0.0 0.0 10.0)))
  (if (== OtherActor _returnvalue)
    (message `/Game/SceneManagement/BPI_SceneManager.CheckpointPlayerTransform` (`self.SceneManager`) (`KismetMathLibrary.MakeTransform` _returnvalue_2 _returnvalue_rotation _returnvalue_scale))
    (`KismetSystemLibrary.PrintString` (`KismetStringLibrary.Conv_VectorToString` _returnvalue_2))))

(fn `UserConstructionScript`)