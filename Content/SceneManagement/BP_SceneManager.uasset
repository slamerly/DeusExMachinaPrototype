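; Scene manager that streams the game's sublevels, loading one scene from the Levels list at a time.
; Transitions save tagged actors, animate curtains and spotlights, swap levels, restore state and teleport the player to the matching BP_TriggerNextScene start.
; It also updates the player controller's moving manager and persists the scene index, applying game-instance load steps once per scene.
; Debug keys and quick-change events skip animations for scene switching, spawn-point teleports and save/load.
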(event OnSave(BPAC_Saver)
  (params (SaveGame :type Save%20Game%20Object%20Reference))
  ;[1 1 1] Save Instance
  (bind _asbp_save_instance (Utilities|Casting|CastToBP_SaveInstance SaveGame))
  (Variables|/Game/Save/BP_SaveInstance.BP_SaveInstance_C|SetStructSceneManager _asbp_save_instance (Utilities|Struct|MakeSTR_Save_SceneManager (Variables|Default|GetCurrentLevelIndex)))
  (Save|SavingScene))

(event OnLoad(BPAC_Saver)
  (params (SaveGame :type Save%20Game%20Object%20Reference))
  ;[1 1 1] Save Instance
  (bind _asbp_save_instance (Utilities|Casting|CastToBP_SaveInstance SaveGame))
  (CallFunction|LoadSaveInstance (.currentindexlevel (Variables|/Game/Save/BP_SaveInstance.BP_SaveInstance_C|GetStructSceneManager _asbp_save_instance))))

(event OnLoadGameInstanceScene(BPAC_Saver)
  (params (LoadStep :type STR%20Game%20Instance%20Structure) (Step :type Integer))
  (bind (_player _scenemanager) (Utilities|Struct|BreakSTR_GameInstance LoadStep))
  (bind _sceneloadstep (Variables|Step|GetSceneLoadStep))
  ;[1 1 1] Save Instance
  (Variables|Step|SetStep Step)
  (for (_ _array_index) _sceneloadstep
    (Utilities|Array|SetArrayElem _sceneloadstep _array_index false))
  (CallFunction|QuickChangeLevel (Utilities|Struct|BreakSTR_Save_SceneManager _scenemanager) false)
  (Transformation|SetActorTransform (Game|Player|GetPlayerPawn 0) (Utilities|Struct|BreakSTR_Save_Player _player)))

(event Custom|ChangeLevel
  (params (Next%20Level :type World%20Soft%20Object%20Reference%20%28by%20ref%29) (TargetID :type Integer))
  ;[1 1 1] Change Level
  (Variables|ChangeLevel|SetTarget%20ID TargetID)
  (if (Utilities|Array|ContainsItem (Variables|Default|GetLevels) Next%20Level)
    (bind _durationanimation (ChangeLevel|BeforeLevelChange (Variables|Default|GetCurrentLevelIndex)))
    (Utilities|FlowControl|Delay (+ _durationanimation 0.25))
    (bind _output_get (Variables|ChangeLevel|SetSaveCurrentLevelIndex (Variables|Default|GetCurrentLevelIndex)))
    (Class|GameplayStatics|UnloadStreamLevelbySoftObjectPtr (Utilities|Array|Get(acopy) (Variables|Default|GetLevels) _output_get) true)
    (Variables|Default|SetCurrentLevelIndex (Utilities|Array|FindItem (Variables|Default|GetLevels) Next%20Level))
    (Class|GameplayStatics|LoadStreamLevelbySoftObjectPtr Next%20Level true true)
    (bind _durationanimation_2 (ChangeLevel|AfterLevelChange (Variables|ChangeLevel|GetSaveCurrentLevelIndex)))
    (Utilities|FlowControl|Delay _durationanimation_2)
    (Input|SetIgnoreMoveInput (Game|GetPlayerController 0) false)
    (else
      ;;[1 0 0 0.33] Error report
      (Development|PrintString (Utilities|String|ToString(Text) (Utilities|Text|FormatText "Next Scene not contains in BP_SceneManager's Levels array")) true true "(R=1.000000,G=0.000000,B=0.000000,A=1.000000)" 1.2e+03))))

(event Custom|CurtainsAnimation
  (params (IsOpen :type Boolean))
  (bind _curtainsinitialposition (Variables|ChangeLevel|Curtains|GetCurtainsInitialPosition))
  (bind _curtains (Variables|ChangeLevel|GetCurtains))
  (bind _curtainsinitialposition_2 (Variables|ChangeLevel|Curtains|GetCurtainsInitialPosition))
  (bind _curtains_2 (Variables|ChangeLevel|GetCurtains))
  (bind _output (Utilities|Array|Get(acopy) _curtainsinitialposition_2))
  (bind _output_2 (Utilities|Array|Get(acopy) _curtains_2))
  (bind _output_3 (Utilities|Array|Get(acopy) _curtainsinitialposition 1))
  (bind _output_4 (Utilities|Array|Get(acopy) _curtains 1))
  (bind _returnvalue (Transformation|GetActorLocation _output_4))
  (bind _returnvalue_2 (Transformation|GetActorLocation _output_2))
  ;[1 1 1] Animations Change Level
  ;;[1 0.25 0 0.33] Curtains Animation
  (if IsOpen
    (bind _newtrack_0 (Timeline|T_CurtainAnim PlayFromStart)
      (:Update
        (Transformation|SetActorLocation _output_2 (Math|Vector|MakeVector (.x _returnvalue_2) (Math|Float|Lerp (.y _output) (+ (.y _output) (Variables|ChangeLevel|Curtains|GetCurtainsDistanceFinalPos)) (Math|Curves|GetFloatValue (Variables|ChangeLevel|Curtains|GetCurveCurtainAnimation) _newtrack_0)) (.z _returnvalue_2)) false false)
        (Transformation|SetActorLocation _output_4 (Math|Vector|MakeVector (.x _returnvalue) (Math|Float|Lerp (.y _output_3) (- (.y _output_3) (Variables|ChangeLevel|Curtains|GetCurtainsDistanceFinalPos)) (Math|Curves|GetFloatValue (Variables|ChangeLevel|Curtains|GetCurveCurtainAnimation) _newtrack_0)) (.z _returnvalue)) false false)))
    (else
      (Timeline|T_CurtainAnim ReverseFromEnd))))

(event Custom|LightsInteraction
  (params (LightOn :type Boolean) (Lights :type Array%20of%20Spot%20Light%20Object%20References) (LightsIntesity :type Array%20of%20Floats%20%28double-precision%29))
  ;[1 1 1] Animations Change Level
  ;;[1 1 0 0.33] Lights Interaction
  (if (Utilities|Array|IsNotEmpty Lights)
    (if LightOn
      (bind _newtrack_0 (Timeline|T_LightsInteraction PlayFromStart)
        (:Update
          (for (_array_element _array_index) Lights
            (Rendering|Components|Light|SetIntensity (Variables|/Script/Engine.SpotLight|GetSpotLightComponent _array_element) (Math|Float|Lerp (Utilities|Array|Get(acopy) LightsIntesity _array_index) 0.0 (Math|Curves|GetFloatValue (Variables|ChangeLevel|Lights|GetCurveLightsInteraction) _newtrack_0))))))
      (elif (Variables|ChangeLevel|GetCurtainsAnimated)
        (Utilities|FlowControl|Delay 0.2)
        (Timeline|T_LightsInteraction ReverseFromEnd)
        (else
          (Timeline|T_LightsInteraction ReverseFromEnd))))))

(event Custom|LoadSaveInstance
  (params (IndexLevel :type Integer))
  (bind _levels (Variables|Default|GetLevels))
  (bind _output (Utilities|Array|Get(acopy) _levels IndexLevel))
  ;[1 1 1] Load save instance
  (if (Utilities|Array|ContainsItem (Variables|Default|GetLevels) _output)
    (ChangeLevel|Quick|BeforeQuickLevelChange false)
    (Class|GameplayStatics|UnloadStreamLevelbySoftObjectPtr (Utilities|Array|Get(acopy) (Variables|Default|GetLevels) (Variables|Default|GetCurrentLevelIndex)) true)
    (bind _output_get (Variables|Default|SetCurrentLevelIndex (Utilities|Array|FindItem (Variables|Default|GetLevels) _output)))
    (Class|GameplayStatics|LoadStreamLevelbySoftObjectPtr _output true true)
    (bind _durationanimation (ChangeLevel|AfterLevelChange _output_get))
    (Utilities|FlowControl|Delay _durationanimation)))

(event Custom|QuickSpawnPoint
  (params (IndexPoint :type Integer))
  (bind _triggersnextscene (Variables|ChangeLevel|Quick|GetTriggersNextScene))
  (bind _output (Utilities|Array|Get(acopy) _triggersnextscene IndexPoint))
  (bind _startscene (Variables|/Game/SceneManagement/BP_TriggerNextScene.BP_TriggerNextScene_C|GetStartScene _output))
  ;[1 1 1] Quick Teleport Spawn Point
  (Game|SetGamePaused false)
  (Utilities|IsValid _startscene
    (:Is%20Valid
      (Transformation|SetActorLocation (Game|Player|GetPlayerPawn 0) (Transformation|GetActorLocation _startscene) false true)
      (Game|SetGamePaused true))))

(event Custom|QuickChangeLevel
  (params (IndexLevel :type Integer) (WithSave :type Boolean))
  (bind _levels (Variables|Default|GetLevels))
  (bind _output (Utilities|Array|Get(acopy) _levels IndexLevel))
  ;[1 1 1] Quick Change Level
  (if (Utilities|Array|ContainsItem (Variables|Default|GetLevels) _output)
    (Game|SetGamePaused false)
    (ChangeLevel|Quick|BeforeQuickLevelChange WithSave)
    (Class|GameplayStatics|UnloadStreamLevelbySoftObjectPtr (Utilities|Array|Get(acopy) (Variables|Default|GetLevels) (Variables|Default|GetCurrentLevelIndex)) true)
    (Variables|Default|SetCurrentLevelIndex (Utilities|Array|FindItem (Variables|Default|GetLevels) _output))
    (Class|GameplayStatics|LoadStreamLevelbySoftObjectPtr _output true true)
    (ChangeLevel|Quick|AfterQuickLevelChange WithSave)
    (Game|SetGamePaused true)))

(event EventBeginPlay
  (bind _curtains (Variables|ChangeLevel|GetCurtains))
  (Utilities|FlowControl|Sequence
    (:then_0
      (bind _asbppc_player (Utilities|Casting|CastToBPPC_Player (Game|GetPlayerController 0)))
      (Variables|Default|SetPlayerControllerRef _asbppc_player))
    (:then_1
      ;[1 1 1] Load first level in list at begin play
      (Class|GameplayStatics|LoadStreamLevelbySoftObjectPtr (Utilities|Array|Get(acopy) (Variables|Default|GetLevels)) true true)
      (bind _returnvalue (Class|LevelUtilitiesFunctions|GetActorOfClassinSublevel (Utilities|Array|Get(acopy) (Variables|Default|GetLevels)) "/Game/SceneManagement/BP_SceneMovingManager.BP_SceneMovingManager_C"))
      (Variables|/Game/Player/BPPC_Player.BPPC_Player_C|SetCurrentMovingManager (Variables|Default|GetPlayerControllerRef) _returnvalue)
      ;[1 0.14 0 0.33] Curatins verifications
      (Development|PrintString (Utilities|String|ToString(Boolean) (Utilities|IsValid _returnvalue)))
      (if (Utilities|Array|IsNotEmpty (Variables|ChangeLevel|GetCurtains))
        (if (> (.y (Transformation|GetActorLocation (Utilities|Array|Get(acopy) (Variables|ChangeLevel|GetCurtains)))) (.y (Transformation|GetActorLocation (Variables|Default|GetSceneCenter))))
          (Utilities|Array|Reverse _curtains))
        (for (_array_element _array_index) _curtains
          (Utilities|Array|SetArrayElem (Variables|ChangeLevel|Curtains|GetCurtainsInitialPosition) _array_index (Transformation|GetActorLocation _array_element)))
        (Components|Timeline|SetPlayRate (Variables|Default|GetT_CurtainAnim) (Variables|ChangeLevel|Curtains|GetCurtainAnimationPlayRate))
        (Components|Timeline|SetPlayRate (Variables|Default|GetT_LightsInteraction) (Variables|ChangeLevel|Lights|GetLightsInteractionPlayRate))
        (ChangeLevel|Quick|UpdateListSpawnPointsDebug)
        (while (< (Utilities|Array|Length (Variables|Step|GetSceneLoadStep)) (Utilities|Array|Length (Variables|Default|GetLevels)))
          (Utilities|Array|Add (Variables|Step|GetSceneLoadStep) false))
        (else
          (Development|PrintText "Curtains don't setup in BP_SceneManager" true true "(R=1.000000,G=0.000000,B=0.000000,A=1.000000)" 1.2e+03))))))

(event Input|KeyboardEvents|DebugKeyCtrlLeft
  (params (Key :type Key%20Structure :default "None") (ActionValue :type Input%20Action%20Value%20Structure))
  ;[1 0.39 0 0.33] Debug
  ;;[1 1 1] Debug quick switch to the previous scene in list
  (:Pressed
    (ChangeLevel|Quick|BeforeQuickLevelChange true)
    (Class|GameplayStatics|UnloadStreamLevelbySoftObjectPtr (Utilities|Array|Get(acopy) (Variables|Default|GetLevels) (Variables|Default|GetCurrentLevelIndex)) true)
    (bind _new_level_index (ChangeLevel|ChangeLevelIndex false))
    (Class|GameplayStatics|LoadStreamLevelbySoftObjectPtr (Utilities|Array|Get(acopy) (Variables|Default|GetLevels) _new_level_index) true true)
    (Save|LoadingScene)))

(event Input|KeyboardEvents|DebugKeyCtrlRight
  (params (Key :type Key%20Structure :default "None") (ActionValue :type Input%20Action%20Value%20Structure))
  ;[1 0.39 0 0.33] Debug
  ;;[1 1 1] Debug quick switch to the next scene in list
  (:Pressed
    (ChangeLevel|Quick|BeforeQuickLevelChange true)
    (Class|GameplayStatics|UnloadStreamLevelbySoftObjectPtr (Utilities|Array|Get(acopy) (Variables|Default|GetLevels) (Variables|Default|GetCurrentLevelIndex)) true)
    (bind _new_level_index (ChangeLevel|ChangeLevelIndex true))
    (Class|GameplayStatics|LoadStreamLevelbySoftObjectPtr (Utilities|Array|Get(acopy) (Variables|Default|GetLevels) _new_level_index) true true)
    (Save|LoadingScene)))

(event Input|KeyboardEvents|DebugKeyCtrlT
  (params (Key :type Key%20Structure :default "None") (ActionValue :type Input%20Action%20Value%20Structure))
  ;[1 0.39 0 0.33] Debug
  ;;[1 1 1] Debug move platforms
  (:Pressed
    (bind _returnvalue (Class|LevelUtilitiesFunctions|GetActorOfClassinSublevel (Utilities|Array|Get(acopy) (Variables|Default|GetLevels) (Variables|Default|GetCurrentLevelIndex)) "/Game/SceneManagement/BP_SceneMovingManager.BP_SceneMovingManager_C"))
    (Utilities|IsValid _returnvalue
      (:Is%20Valid
        (Default|DebugMovePlatform _returnvalue (Transformation|GetActorLocation (Game|GetPlayerCharacter 0)))))))

(event Input|KeyboardEvents|DebugKeyN
  (params (Key :type Key%20Structure :default "None") (ActionValue :type Input%20Action%20Value%20Structure))
  ;[1 0.39 0 0.33] Debug
  ;;[1 1 1] Debug Save
  (:Pressed
    (bind _asbp_gi_deus_ex (Utilities|Casting|CastToBP_GI_DeusEx (Game|GetGameInstance)))
    (Default|GlobalLoad _asbp_gi_deus_ex)))

(event Input|KeyboardEvents|DebugKeyB
  (params (Key :type Key%20Structure :default "None") (ActionValue :type Input%20Action%20Value%20Structure))
  ;[1 0.39 0 0.33] Debug
  ;;[1 1 1] Debug Save
  (:Pressed
    (bind _asbp_gi_deus_ex (Utilities|Casting|CastToBP_GI_DeusEx (Game|GetGameInstance)))
    (Default|GlobalSave _asbp_gi_deus_ex)))

(event Input|KeyboardEvents|DebugKeyCtrlR
  (params (Key :type Key%20Structure :default "None") (ActionValue :type Input%20Action%20Value%20Structure))
  ;[1 0.39 0 0.33] Debug
  ;;[1 1 1] Debug rotate supports
  (:Pressed
    (bind _returnvalue (Class|LevelUtilitiesFunctions|GetActorOfClassinSublevel (Utilities|Array|Get(acopy) (Variables|Default|GetLevels) (Variables|Default|GetCurrentLevelIndex)) "/Game/SceneManagement/BP_SceneMovingManager.BP_SceneMovingManager_C"))
    (Utilities|IsValid _returnvalue
      (:Is%20Valid
        (Default|DebugRotateSupport _returnvalue (Transformation|GetActorLocation (Game|GetPlayerCharacter 0)))))))

(fn ConstructionScript)

(fn ChangeLevelIndex
  (params (bIncreasing :type Boolean))
  (if bIncreasing
    ;[1 1 1] Increase
    (if (== (+ (Variables|Default|GetCurrentLevelIndex) 1) (Utilities|Array|Length (Variables|Default|GetLevels)))
      (bind _output_get (Variables|Default|SetCurrentLevelIndex 0))
      (return _output_get)
      (else
        (bind _result (Math|Integer|IncrementInt (Variables|Default|GetCurrentLevelIndex))
          (:%20%20
            (return _result)))))
    (else
      ;[1 1 1] Decrease
      (if (== (- (Variables|Default|GetCurrentLevelIndex) 1) -1)
        (bind _output_get_2 (Variables|Default|SetCurrentLevelIndex (- (Utilities|Array|Length (Variables|Default|GetLevels)) 1)))
        (return _output_get_2)
        (else
          (bind _result_2 (Math|Integer|DecrementInt (Variables|Default|GetCurrentLevelIndex))
            (:%20%20
              (return _result_2))))))))

(fn AfterLevelChange
  (params (CurrentLevelIndex :type Integer))
  (bind _t_lightsinteraction (Variables|Default|GetT_LightsInteraction))
  (bind _t_curtainanim (Variables|Default|GetT_CurtainAnim))
  (bind _lightsintensity (LocalVariables|GetLightsIntensity))
  (bind _returnvalue (Components|Timeline|GetTimelineLength _t_lightsinteraction))
  (bind _returnvalue_2 (Components|Timeline|GetTimelineLength _t_curtainanim))
  (bind _returnvalue_3 (Components|Animation|GetPlayRate _t_curtainanim))
  (bind _returnvalue_4 (Components|Animation|GetPlayRate _t_lightsinteraction))
  (bind _returnvalue_5 (- 1.0 _returnvalue_4))
  (bind _returnvalue_6 (- 1.0 _returnvalue_3))
  (bind _returnvalue_7 (* _returnvalue_2 _returnvalue_6))
  (bind _returnvalue_8 (* _returnvalue _returnvalue_5))
  (bind _returnvalue_9 (+ _returnvalue_2 _returnvalue_7))
  (bind _returnvalue_10 (+ _returnvalue _returnvalue_8))
  (Utilities|FlowControl|Sequence
    (:then_0
      (bind _output_get (LocalVariables|SetLevelIndex CurrentLevelIndex))
      (Save|LoadingScene)
      ;[1 1 1] If the scene contains many transistion, select the good transition
      (bind _outactors (Actor|GetAllActorsOfClass "/Game/SceneManagement/BP_TriggerNextScene.BP_TriggerNextScene_C"))
      (for _array_element _outactors
        (if (and (== (Variables|/Game/SceneManagement/BP_TriggerNextScene.BP_TriggerNextScene_C|GetTargetScene _array_element) (Utilities|Array|Get(acopy) (Variables|Default|GetLevels) _output_get)) (== (Variables|ChangeLevel|GetTarget%20ID) (Variables|/Game/SceneManagement/BP_TriggerNextScene.BP_TriggerNextScene_C|GetID _array_element)))
          ;;[1 1 1] Teleport player to the start location
          (Utilities|IsValid (Variables|/Game/SceneManagement/BP_TriggerNextScene.BP_TriggerNextScene_C|GetStartScene _array_element)
            (:Is%20Valid
              (Transformation|SetActorLocation (Game|Player|GetPlayerPawn 0) (Transformation|GetActorLocation (Variables|/Game/SceneManagement/BP_TriggerNextScene.BP_TriggerNextScene_C|GetStartScene _array_element)) false true))
            (:Is%20Not%20Valid
              ;[1 0 0] Message Error
              (Development|PrintString (Utilities|String|ToString(Text) (Utilities|Text|FormatText "StartScene is empty in {BP}" (Class|KismetSystemLibrary|GetPathName _array_element))) true true "(R=1.000000,G=0.000000,B=0.000000,A=1.000000)" 1.2e+03)))))
      ;[1 1 1] Animation
      (if (Variables|ChangeLevel|GetCurtainsAnimated)
        (CallFunction|CurtainsAnimation false))
      (if (Variables|ChangeLevel|GetLightsAnimated)
        (for _array_element_2 (Variables|/Game/SceneManagement/BP_TriggerNextScene.BP_TriggerNextScene_C|GetLights _array_element)
          (Utilities|Array|Add _lightsintensity (Variables|/Script/Engine.LightComponentBase|GetIntensity (Variables|/Script/Engine.SpotLight|GetSpotLightComponent _array_element_2))))
        (CallFunction|LightsInteraction false (Variables|/Game/SceneManagement/BP_TriggerNextScene.BP_TriggerNextScene_C|GetLights _array_element) _lightsintensity))
      (if (Variables|ChangeLevel|GetCurtainsAnimated)
        (if (Variables|ChangeLevel|GetLightsAnimated)
          (if (> _returnvalue_10 _returnvalue_9)
            (return _returnvalue_10)
            (else
              (return _returnvalue_9)))
          (else
            (return _returnvalue_9)))
        (elif (Variables|ChangeLevel|GetLightsAnimated)
          (return _returnvalue_10))))
    (:then_1
      (bind _returnvalue_11 (Class|LevelUtilitiesFunctions|GetActorOfClassinSublevel (Utilities|Array|Get(acopy) (Variables|Default|GetLevels) (Variables|Default|GetCurrentLevelIndex)) "/Game/SceneManagement/BP_SceneMovingManager.BP_SceneMovingManager_C"))
      (Variables|/Game/Player/BPPC_Player.BPPC_Player_C|SetCurrentMovingManager (Variables|Default|GetPlayerControllerRef) _returnvalue_11))))

(fn BeforeLevelChange
  (params (CurrentLevelIndex :type Integer))
  (bind _t_lightsinteraction (Variables|Default|GetT_LightsInteraction))
  (bind _t_curtainanim (Variables|Default|GetT_CurtainAnim))
  (bind _returnvalue (Components|Timeline|GetTimelineLength _t_lightsinteraction))
  (bind _returnvalue_2 (Components|Timeline|GetTimelineLength _t_curtainanim))
  (bind _returnvalue_3 (Components|Animation|GetPlayRate _t_curtainanim))
  (bind _returnvalue_4 (Components|Animation|GetPlayRate _t_lightsinteraction))
  (bind _returnvalue_5 (- 1.0 _returnvalue_4))
  (bind _returnvalue_6 (- 1.0 _returnvalue_3))
  (bind _returnvalue_7 (* _returnvalue_2 _returnvalue_6))
  (bind _returnvalue_8 (* _returnvalue _returnvalue_5))
  (bind _returnvalue_9 (+ _returnvalue_2 _returnvalue_7))
  (bind _returnvalue_10 (+ _returnvalue _returnvalue_8))
  (Save|SavingScene)
  (Input|SetIgnoreMoveInput (Game|GetPlayerController 0) true)
  (if (Variables|ChangeLevel|GetLightsAnimated)
    (bind (_spotlights _lightsintensity) (ChangeLevel|Lights|GetSpotLights CurrentLevelIndex))
    ;[1 1 1] Animations
    (CallFunction|LightsInteraction true _spotlights _lightsintensity))
  (if (Variables|ChangeLevel|GetCurtainsAnimated)
    (CallFunction|CurtainsAnimation true))
  (if (> _returnvalue_10 _returnvalue_9)
    (return _returnvalue_10)
    (else
      (return _returnvalue_9))))

(fn GetSpotLights
  (params (LevelIndex :type Integer))
  (bind _outactors (Class|LevelUtilitiesFunctions|GetAllActorsOfClassinSublevel (Utilities|Array|Get(acopy) (Variables|Default|GetLevels) LevelIndex) "/Script/Engine.SpotLight"))
  (bind _output_get (LocalVariables|SetSpots%20Light _outactors))
  (for _array_element _output_get
    (Utilities|Array|Add (LocalVariables|GetLightsInten) (Variables|/Script/Engine.LightComponentBase|GetIntensity (Variables|/Script/Engine.SpotLight|GetSpotLightComponent _array_element))))
  (return (LocalVariables|GetSpots%20Light) (LocalVariables|GetLightsInten)))

(fn AfterQuickLevelChange
  (params (Saving :type Boolean))
  (bind _triggersnextscene (Variables|ChangeLevel|Quick|GetTriggersNextScene))
  (bind _output (Utilities|Array|Get(acopy) _triggersnextscene))
  (bind _startscene (Variables|/Game/SceneManagement/BP_TriggerNextScene.BP_TriggerNextScene_C|GetStartScene _output))
  (Utilities|FlowControl|Sequence
    (:then_0
      (if Saving
        (Save|LoadingScene)
        (elif (and (!= (Variables|Step|GetStep) -1) (not (Utilities|Array|Get(acopy) (Variables|Step|GetSceneLoadStep) (Variables|Default|GetCurrentLevelIndex))))
          (Step|LoadingStep (Variables|Step|GetStep))
          (Utilities|Array|SetArrayElem (Variables|Step|GetSceneLoadStep) (Variables|Default|GetCurrentLevelIndex) true)))
      (ChangeLevel|Quick|UpdateListSpawnPointsDebug)
      ;[1 1 1] Teleport player to the start location
      (Utilities|IsValid _startscene
        (:Is%20Valid
          (Transformation|SetActorLocation (Game|Player|GetPlayerPawn 0) (Transformation|GetActorLocation _startscene) false true))
        (:Is%20Not%20Valid
          ;[1 0 0] Message Error
          (Development|PrintString (Utilities|String|ToString(Text) (Utilities|Text|FormatText "StartScene is empty in {BP}" (Class|KismetSystemLibrary|GetPathName _output))) true true "(R=1.000000,G=0.000000,B=0.000000,A=1.000000)" 1.2e+03))))
    (:then_1
      (bind _returnvalue (Class|LevelUtilitiesFunctions|GetActorOfClassinSublevel (Utilities|Array|Get(acopy) (Variables|Default|GetLevels) (Variables|Default|GetCurrentLevelIndex)) "/Game/SceneManagement/BP_SceneMovingManager.BP_SceneMovingManager_C"))
      (Variables|/Game/Player/BPPC_Player.BPPC_Player_C|SetCurrentMovingManager (Variables|Default|GetPlayerControllerRef) _returnvalue))))

(fn GetNumberSpawPoints
  (return (Utilities|Array|Length (Variables|ChangeLevel|Quick|GetTriggersNextScene))))

(fn UpdateListSpawnPointsDebug
  (Utilities|Array|Clear (Variables|ChangeLevel|Quick|GetTriggersNextScene))
  (bind _outactors (Actor|GetAllActorsOfClass "/Game/SceneManagement/BP_TriggerNextScene.BP_TriggerNextScene_C"))
  (for _array_element _outactors
    (Utilities|Array|Add (Variables|ChangeLevel|Quick|GetTriggersNextScene) _array_element))
  (bind _foundwidgets (Class|WidgetBlueprintLibrary|GetAllWidgetswithInterface "/Game/Debug/BPI_Debug.BPI_Debug_C" false))
  (Class|BPIDebug|UpdateListSpawnPoints(Message) (Utilities|Array|Get(acopy) _foundwidgets) (Utilities|Array|Length (Variables|ChangeLevel|Quick|GetTriggersNextScene))))

(fn BeforeQuickLevelChange
  (params (Saving :type Boolean))
  (if Saving
    (Save|SavingScene)))

(fn SavingScene
  (bind _outactors (Actor|GetAllActorswithTag "SaveScene"))
  (for _array_element _outactors
    (Class|BPISaver|Save(Message) (Utilities|Array|Get(acopy) (Class|Actor|GetComponentsbyInterface _array_element "/Game/Save/BPI_Saver.BPI_Saver_C"))))
  (Development|PrintString "SaveScene" true true "(R=0.000000,G=0.250000,B=1.000000,A=1.000000)"))

(fn LoadingScene
  (if (and (!= (Variables|Step|GetStep) -1) (not (Utilities|Array|Get(acopy) (Variables|Step|GetSceneLoadStep) (Variables|Default|GetCurrentLevelIndex))))
    (Step|LoadingStep (Variables|Step|GetStep))
    (Utilities|Array|SetArrayElem (Variables|Step|GetSceneLoadStep) (Variables|Default|GetCurrentLevelIndex) true)
    (else
      (bind _outactors (Actor|GetAllActorswithTag "SaveScene"))
      (for _array_element _outactors
        (Class|BPISaver|Load(Message) (Utilities|Array|Get(acopy) (Class|Actor|GetComponentsbyInterface _array_element "/Game/Save/BPI_Saver.BPI_Saver_C"))))
      (Development|PrintString "LoadScene" true true "(R=0.000000,G=0.250000,B=1.000000,A=1.000000)"))))

(fn GetAllActorsNamewithSave
  (bind _outactors (Actor|GetAllActorswithTag "SaveScene"))
  (for _array_element _outactors
    (Development|PrintString (Utilities|GetDisplayName _array_element) true true "(R=0.000000,G=0.660000,B=1.000000,A=1.000000)" 15.0)))

(fn LoadingStep
  (params (Step :type Integer))
  (bind _outactors (Actor|GetAllActorswithTag "SaveScene"))
  (for _array_element _outactors
    (Class|BPISaver|LoadStep(Message) (Utilities|Array|Get(acopy) (Class|Actor|GetComponentsbyInterface _array_element "/Game/Save/BPI_Saver.BPI_Saver_C")) Step))
  (Development|PrintString "LoadStep" true true "(R=0.250000,G=0.250000,B=1.000000,A=1.000000)"))

(fn GetCurrentIndexScene
  (return (Variables|Default|GetCurrentLevelIndex)))