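; Scene manager that tracks the level's rotation supports and moving platforms and resolves which one the player is in range of.
; On BeginPlay it gathers both actor types, also merging them into a shared MovingObjects list.
; Searches take the first in-range object, then recurse through its children to the deepest in-range descendant.
; SearchMovingObject returns that object, while debug functions trigger a support's debug rotation or a platform's player interaction.
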(event `self.ReceiveBeginPlay`
  (bind _returnvalue (`self.GetLevel`))
  (`|ExecutionSequence`
    (:`then_0`
      ;[0.3997 0.6132 1] Retrieve Rotation Supports and Moving Platforms
      (bind _outactors (`LevelUtilitiesFunctions.GetAllActorsOfClassInLevel` _returnvalue "/Game/GPE/Moving/Rotation/BP_RotationSupport.BP_RotationSupport_C"))
      (bind _output_get (set `self.RotationSupports` _outactors))
      (set `self.MovingObjects` _output_get))
    (:`then_1`
      (bind _outactors_2 (`LevelUtilitiesFunctions.GetAllActorsOfClassInLevel` _returnvalue "/Game/GPE/Moving/MovingPlatforms/BP_MovingPlatform.BP_MovingPlatform_C"))
      (bind _output_get_2 (set `self.MovingPlatforms` _outactors_2))
      (for _array_element _output_get_2
        (`KismetArrayLibrary.Array_Add` (`self.MovingObjects`) _array_element)))))

(fn `Debug Move Platform`
  (params (PlayerPosition :type "Vector Structure"))
  (if (> (`KismetArrayLibrary.Array_Length` (`self.MovingPlatforms`)) 0)
    (for _array_element (`self.MovingPlatforms`)
      (if (`/Game/GPE/Moving/BP_MovingBase.GetPlayerInRange` _array_element PlayerPosition)
        (`self.SearchChildrensPlatforms` _array_element PlayerPosition)
        (return)))))

(fn `DebugRotateSupport`
  (params (PlayerPosition :type "Vector Structure"))
  (if (> (`KismetArrayLibrary.Array_Length` (`self.RotationSupports`)) 0)
    (for _array_element (`self.RotationSupports`)
      (if (`/Game/GPE/Moving/BP_MovingBase.GetPlayerInRange` _array_element PlayerPosition)
        (`self.SearchChildrenSupports` _array_element PlayerPosition)
        (return)))))

(fn `Search Moving Object`
  (params (PlayerPos :type "Vector Structure"))
  (returns (ObjectFound :type Boolean) (MovingObject :type "/Game/GPE/Moving/BP_MovingBase Object Reference"))
  (locals (NewLocalVar :type Boolean :default false))
  (if (`KismetArrayLibrary.Array_IsNotEmpty` (`self.MovingObjects`))
    (for _array_element (`self.MovingObjects`)
      (if (`/Game/GPE/Moving/BP_MovingBase.GetPlayerInRange` _array_element (`local.PlayerPos`))
        (bind _foundmovingobject (`self.SearchChildMovingObject` _array_element (`local.PlayerPos`)))
        (return true _foundmovingobject)))
    (return false null)
    (else
      (return false null))))

(fn `SearchChildMovingObject`
  (params (MovingObject :type "/Game/GPE/Moving/BP_MovingBase Object Reference") (PlayerPos :type "Vector Structure"))
  (returns (FoundMovingObject :type "/Game/GPE/Moving/BP_MovingBase Object Reference"))
  (for _array_element (`/Game/GPE/Moving/BP_MovingBase.MovableChilds` MovingObject)
    (bind (_ismovingobject _selfmovingobject) (`/Game/GPE/Moving/BPAC_MovableObject.IsSelfMovingObject` _array_element))
    (if _ismovingobject
      (if (`/Game/GPE/Moving/BP_MovingBase.GetPlayerInRange` _selfmovingobject (`local.PlayerPos`))
        (bind _foundmovingobject (`self.SearchChildMovingObject` _selfmovingobject (`local.PlayerPos`)))
        (return _foundmovingobject))))
  (return MovingObject))

(fn `SearchChildrensPlatforms`
  (params (Platform :type "/Game/GPE/Moving/MovingPlatforms/BP_MovingPlatform Object Reference") (PlayerPosition :type "Vector Structure"))
  (bind _platformchilds (`/Game/GPE/Moving/MovingPlatforms/BP_MovingPlatform.GetMovingPlatformsChilds` Platform))
  (for _array_element _platformchilds
    (if (`/Game/GPE/Moving/BP_MovingBase.GetPlayerInRange` _array_element PlayerPosition)
      (`self.SearchChildrensPlatforms` _array_element PlayerPosition)
      (return)))
  (`/Game/GPE/Moving/MovingPlatforms/BP_MovingPlatform.PlayerInteraction` Platform)
  (return))

(fn `SearchChildrenSupports`
  (params (Support :type "/Game/GPE/Moving/Rotation/BP_RotationSupport Object Reference") (PlayerPosition :type "Vector Structure"))
  (bind _supportschilds (`/Game/GPE/Moving/Rotation/BP_RotationSupport.GetRotationSupportChilds` Support))
  (for _array_element _supportschilds
    (if (`/Game/GPE/Moving/BP_MovingBase.GetPlayerInRange` _array_element PlayerPosition)
      (`self.SearchChildrenSupports` _array_element PlayerPosition)
      (return)))
  (`/Game/GPE/Moving/Rotation/BP_RotationSupport.StartStandardRotation` Support (`/Game/GPE/Moving/Rotation/BP_RotationSupport.DebugRotationAngle` Support) (`/Game/GPE/Moving/Rotation/BP_RotationSupport.DebugRotationDuration` Support) (`/Game/GPE/Moving/Rotation/BP_RotationSupport.DebugRotationCurve` Support))
  (return))

(fn `UserConstructionScript`)