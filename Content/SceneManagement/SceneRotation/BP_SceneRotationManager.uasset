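; BP_SceneRotationManager is a manager Blueprint that triggers rotation of scene objects and rotation supports.
; RotateScene180 tells each listed actor's BPAC_SceneRotationObject component to rotate around a given center, using a hardcoded 50-degree angle despite its name.
; DebugRotateSupport starts the first RotationSupport within range of the player using that support's debug settings, printing a warning if none qualifies.
; The event graph and construction script are empty.
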(fn `DebugRotateSupport`
  (params (PlayerPosition :type "Vector Structure"))
  (if (> (`KismetArrayLibrary.Array_Length` (`self.RotationSupports`)) 0)
    (for _array_element (`self.RotationSupports`)
      (if (< (`KismetMathLibrary.Vector_Distance` (`self.K2_GetActorLocation` _array_element) PlayerPosition) (`/Game/GPE/BP_RotationSupport.GetRange` _array_element))
        (`/Game/GPE/BP_RotationSupport.StartRotation` _array_element (`/Game/GPE/BP_RotationSupport.DebugRotationAngle` _array_element) (`/Game/GPE/BP_RotationSupport.DebugRotationDuration` _array_element))
        (return)))
    (`KismetSystemLibrary.PrintText` "The Player was not in range of a Rotation Support." true true (struct :`R` 1.0 :`G` 0.327038 :`A` 1.0) 2.0 "Debug Rotation Log")
    (else
      (`KismetSystemLibrary.PrintText` "The Scene Rotation Manager has no Rotation Support." true true (struct :`R` 1.0 :`G` 0.665043 :`A` 1.0) 2.0 "Debug Rotation Log"))))

(fn `RotateScene180`
  (params (`Scene Center` :type "Actor Object Reference"))
  (for _array_element (`self.SceneActorsToRotate`)
    (`/Game/SceneManagement/SceneRotation/BPAC_SceneRotationObject.StartRotating` (`self.GetComponentByClass` _array_element "/Game/SceneManagement/SceneRotation/BPAC_SceneRotationObject.BPAC_SceneRotationObject_C") `Scene Center` 50.0 1.0)))

(fn `UserConstructionScript`)