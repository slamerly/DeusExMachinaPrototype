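; Controller for selecting and rotating scene rotation supports in layers, mostly disconnected: input handlers are empty and Tick only checks the manager.
; RegisterManager just stores the manager, as its code grouping controller-friendly supports into parent-keyed layers never runs.
; SwitchLayer selects a layer's first support, and SwitchSupport moves the outline highlight.
; Directional navigation scores supports by 2D dot product, then picks the closest among near-best matches, but its caller is unwired.
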(event `self.ReceiveTick`
  (params (DeltaSeconds :type "Float (single-precision)"))
  (`/Engine/EditorBlueprintResources/StandardMacros.IsValid` (`self.CurrentManager`)))

(fn `ClearManager`
  (`/Engine/EditorBlueprintResources/StandardMacros.IsValid` (`self.CurrentManager`)
    (:`Is Valid`
      (set `self.CurrentManager` null)
      (`KismetArrayLibrary.Array_Clear` (`self.RotationsLayers`)))))

(fn `GetControllerFriendlyParent`
  (params (Support :type "/Game/GPE/Moving/Rotation/BP_RotationSupport Object Reference"))
  (returns (Parent :type "/Game/SceneManagement/SceneRotation/BPI_RotationLayerParent Interface") (ParentAsActor :type "Actor Object Reference"))
  (bind _currentmanager (`self.CurrentManager`))
  (return _currentmanager _currentmanager))

(fn `QuerryLayers`
  (params (LayerParent :type "/Game/SceneManagement/SceneRotation/BPI_RotationLayerParent Interface"))
  (returns (LayerFound :type Boolean) (Layer :type "/Game/GPE/Moving/Rotation/STR_RotationLayer Structure"))
  (bind _object (`/Game/SceneManagement/SceneRotation/BPI_RotationLayerParent.GetObject` LayerParent))
  (for _array_element (`self.RotationsLayers`)
    (bind _object_2 (`/Game/SceneManagement/SceneRotation/BPI_RotationLayerParent.GetObject` (`.LayerParent_9_8638C826464859B702EAFB9846790B84` (break `/Game/GPE/Moving/Rotation/STR_RotationLayer` _array_element))))
    (if (== _object_2 _object)
      (return true _array_element)))
  (return false))

(fn `QuerryNavigateSupports`
  (params (QueryDirection :type "Vector2D Structure"))
  (returns (SupportFound :type "/Game/GPE/Moving/Rotation/BP_RotationSupport Object Reference"))
  (locals (SupportsDotProduct :type "Map of /Game/GPE/Moving/Rotation/BP_RotationSupport Object Reference to Float (double-precision)") (BestDotProduct :type "Float (double-precision)" :default -1.0) (ClosestDistance :type "Float (double-precision)" :default 9999999999.0) (BestSupportFound :type "/Game/GPE/Moving/Rotation/BP_RotationSupport Object Reference"))
  (for _array_element (`.RotationSupports_3_6AE13D634EA24E14DCD27EBF0967A781` (break `/Game/GPE/Moving/Rotation/STR_RotationLayer` (`self.CurrentLayer`)))
    (if (!= _array_element (`self.CurrentSupport`))
      (bind _returnvalue (`KismetMathLibrary.DotProduct2D` QueryDirection (`KismetMathLibrary.Conv_VectorToVector2D` (`KismetMathLibrary.Vector_Normal2D` (- (`self.K2_GetActorLocation` _array_element) (`self.K2_GetActorLocation` (`self.CurrentSupport`)))))))
      ;[1 1 1] Dot Product Test
      (if (> _returnvalue (`self.QueryMinDotProduct`))
        (`BlueprintMapLibrary.Map_Add` (`local.SupportsDotProduct`) _array_element _returnvalue)
        (if (> _returnvalue (`local.BestDotProduct`))
          (set `local.BestDotProduct` _returnvalue)))))
  (bind _keys (`BlueprintMapLibrary.Map_Keys` (`local.SupportsDotProduct`)))
  (for _array_element_2 _keys
    (if (>= (`BlueprintMapLibrary.Map_Find` (`local.SupportsDotProduct`) _array_element_2) (- (`local.BestDotProduct`) (`self.QueryDistOverDot`)))
      (bind _returnvalue_2 (`KismetMathLibrary.Vector_Distance2D` (`self.K2_GetActorLocation` _array_element_2) (`self.K2_GetActorLocation` (`self.CurrentSupport`))))
      (if (< _returnvalue_2 (`local.ClosestDistance`))
        (set `local.ClosestDistance` _returnvalue_2)
        (set `local.BestSupportFound` _array_element_2))))
  (return (`local.BestSupportFound`)))

(fn `RegisterManager`
  (params (Manager :type "/Game/SceneManagement/SceneRotation/BP_SceneRotationManager Object Reference"))
  (locals (RotationsSupportsConstructingLayers :type "Map of Actor Object Reference to /Game/GPE/Moving/Rotation/STR_RotationLayer Structure") (CurrentModifyingArray :type "Array of /Game/GPE/Moving/Rotation/BP_RotationSupport Object Reference") (CurrentCheckedSupport :type "/Game/GPE/Moving/Rotation/BP_RotationSupport Object Reference"))
  (`self.ClearManager`)
  (bind _output_get (set `self.CurrentManager` Manager)))

(fn `RotationsInput_LayerDown`)

(fn `RotationsInput_LayerUp`
  (locals (SupportToSwitchIn :type "/Game/GPE/Moving/Rotation/BP_RotationSupport Object Reference")))

(fn `RotationsInput_Navigate`
  (params (`Navigation Direction` :type "Vector2D Structure")))

(fn `RotationsInput_RotateLeft`)

(fn `RotationsInput_RotateRight`)

(fn `SwitchLayer`
  (params (Layer :type "/Game/GPE/Moving/Rotation/STR_RotationLayer Structure"))
  (bind _output_get (set `self.CurrentLayer` Layer))
  (`self.SwitchSupport` (`|GetArrayItem` (`.RotationSupports_3_6AE13D634EA24E14DCD27EBF0967A781` (break `/Game/GPE/Moving/Rotation/STR_RotationLayer` _output_get)))))

(fn `SwitchSupport`
  (params (Support :type "/Game/GPE/Moving/Rotation/BP_RotationSupport Object Reference"))
  (bind _currentsupport (`self.CurrentSupport`))
  (`/Engine/EditorBlueprintResources/StandardMacros.IsValid` _currentsupport
    (:`Is Valid`
      (`/Game/GPE/Moving/Rotation/BP_RotationSupport.SetOutlineVisibility` _currentsupport false))
    (:`Is Not Valid`
      _))
  (bind _output_get (set `self.CurrentSupport` Support))
  (`/Game/GPE/Moving/Rotation/BP_RotationSupport.SetOutlineVisibility` _output_get true))

(fn `UserConstructionScript`)