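; BP_TransitionLVL switches the game to a target level behind a curtain animation and camera fade.
; On BeginPlay it async-loads the BP_SceneManager class and caches that actor from the world.
; Its Transition event blocks player input, tells the scene manager to animate the curtains, removes all widgets and starts a held camera fade.
; After a configurable delay, it opens the target level by object reference.
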(event `self.ReceiveBeginPlay`
  (bind _class (`|LoadAssetClass` "/Game/SceneManagement/BP_SceneManager.BP_SceneManager_C")
    (:`Completed`
      (bind _asactor (castclass `Actor` _class))
      (bind _returnvalue (`GameplayStatics.GetActorOfClass` _asactor))
      (set `self.SceneManager` _returnvalue))))

(event `Transition`
  (message `/Game/Player/BPI_PlayerController.BlockPlayerInputs` (`GameplayStatics.GetPlayerController` 0) "NewEnumerator3")
  (message `/Game/SceneManagement/BPI_SceneManager.CurtainsAnimation` (`self.SceneManager`) true)
  (`WidgetLayoutLibrary.RemoveAllWidgets`)
  (`PlayerCameraManager.StartCameraFade` :`self` (`GameplayStatics.GetPlayerCameraManager` 0) :`ToAlpha` 1.0 :`Duration` 2.0 :`bHoldWhenFinished` true)
  (`KismetSystemLibrary.Delay` (`self.DelayBeforeSwitchLVL`))
  (`GameplayStatics.OpenLevelBySoftObjectPtr` (`self.TargetLevel`)))

(fn `UserConstructionScript`)