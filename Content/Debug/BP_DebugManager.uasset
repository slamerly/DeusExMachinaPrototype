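; BP_DebugManager toggles the debug menu and game pause when the ² key is pressed.
; It tracks the paused state in its own boolean, switching input mode between Game Only and Game and UI along with mouse cursor visibility.
; It reaches the menu by casting the player's HUD to BP_HUD_DeusEx and calling enable or disable on its DebugWidget.
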(event EventBeginPlay)

(event Collision|EventActorBeginOverlap
  (params (OtherActor :type Actor%20Object%20Reference)))

(event EventTick
  (params (DeltaSeconds :type Float%20%28single-precision%29)))

(event Input|KeyboardEvents|DebugKey²
  (params (Key :type Key%20Structure :default "None") (ActionValue :type Input%20Action%20Value%20Structure))
  (bind _returnvalue (Game|GetPlayerController 0))
  (bind _returnvalue_2 (Game|GetPlayerController 0))
  (:Pressed
    (if (Variables|Default|GetbGamePausedaa)
      (Variables|Default|SetbGamePausedaa false)
      (Game|SetGamePaused false)
      (Input|SetInputModeGameOnly _returnvalue false)
      (Variables|/Script/Engine.PlayerController|SetbShowMouseCursor _returnvalue false)
      (bind _asbp_hud_deus_ex (Utilities|Casting|CastToBP_HUD_DeusEx (HUD|GetHUD _returnvalue)))
      (Default|DisableDebugMenu (Variables|/Game/_GameManager/BP_HUD_DeusEx.BP_HUD_DeusEx_C|GetDebugWidget _asbp_hud_deus_ex))
      (else
        (Variables|Default|SetbGamePausedaa true)
        (Game|SetGamePaused true)
        (Input|SetInputModeGameandUI _returnvalue_2 0 "LockOnCapture" false false)
        (Variables|/Script/Engine.PlayerController|SetbShowMouseCursor _returnvalue_2 true)
        (bind _asbp_hud_deus_ex_2 (Utilities|Casting|CastToBP_HUD_DeusEx (HUD|GetHUD _returnvalue_2)))
        (Default|EnableDebugMenu (Variables|/Game/_GameManager/BP_HUD_DeusEx.BP_HUD_DeusEx_C|GetDebugWidget _asbp_hud_deus_ex_2))))))

(fn ConstructionScript)