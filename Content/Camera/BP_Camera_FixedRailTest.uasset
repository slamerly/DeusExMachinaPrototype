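; Test fixed-rail camera that becomes the player's view target on BeginPlay and follows the character along a spline.
; Each tick, the CineCamera eases toward the player's world Y, clamped between the spline's start and point 1, with X and Z locked to the start.
; When the player is at least 350 units above or below, it also eases its yaw toward them, clamped to a narrow range.
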(event `self.ReceiveBeginPlay`
  (`PlayerController.SetViewTargetWithBlend` (`GameplayStatics.GetPlayerController` 0) self 0.0 "VTBlend_Linear" 0.0 false))

(event `self.ReceiveTick`
  (params (DeltaSeconds :type "Float (single-precision)"))
  (bind _cinecamera (`self.CineCamera`))
  (bind (_returnvalue_x _returnvalue_y _returnvalue_z) (`KismetMathLibrary.BreakVector` (`self.K2_GetActorLocation` (`GameplayStatics.GetPlayerCharacter` 0))))
  (bind (_returnvalue_x_2 _returnvalue_y_2 _returnvalue_z_2) (`KismetMathLibrary.BreakVector` (`SceneComponent.K2_GetComponentLocation` (`self.CineCamera`))))
  (bind (_returnvalue_x_3 _returnvalue_y_3 _returnvalue_z_3) (`KismetMathLibrary.BreakVector` (`SplineComponent.GetLocationAtDistanceAlongSpline` (`self.Spline`) 0.0 "World")))
  (bind (_returnvalue_x_4 _returnvalue_y_4) (`KismetMathLibrary.BreakVector` (`self.K2_GetActorLocation` (`GameplayStatics.GetPlayerCharacter` 0))))
  (bind (_returnvalue_x_5 _returnvalue_y_5) (`KismetMathLibrary.BreakVector` (`SceneComponent.K2_GetComponentLocation` (`self.CineCamera`))))
  (bind (_returnvalue_x_6 _returnvalue_y_6) (`KismetMathLibrary.BreakVector` (`KismetMathLibrary.VInterpTo` (`KismetMathLibrary.MakeVector` 0.0 _returnvalue_y_5) (`KismetMathLibrary.MakeVector` 0.0 _returnvalue_y_4) (`GameplayStatics.GetWorldDeltaSeconds`) 1.0)))
  (bind _returnvalue (- _returnvalue_z _returnvalue_z_2))
  (bind (_returnvalue_roll _returnvalue_pitch _returnvalue_yaw) (`KismetMathLibrary.BreakRotator` (`KismetMathLibrary.RInterpTo` (`SceneComponent.K2_GetComponentRotation` _cinecamera) (`KismetMathLibrary.FindLookAtRotation` (`SceneComponent.K2_GetComponentLocation` _cinecamera) (`self.K2_GetActorLocation` (`GameplayStatics.GetPlayerCharacter` 0))) (`GameplayStatics.GetWorldDeltaSeconds`) 1.0)))
  (`SceneComponent.K2_SetWorldLocation` (`self.CineCamera`) (`KismetMathLibrary.MakeVector` _returnvalue_x_3 (`KismetMathLibrary.FClamp` _returnvalue_y_6 _returnvalue_y_3 (.y (.location (`SplineComponent.GetTransformAtSplinePoint` (`self.Spline`) 1 "World" false)))) _returnvalue_z_3) false false)
  (if (<= _returnvalue -350.0)
    (set `self.ConditionOfRotation` true :!label _label)
    (elif (>= _returnvalue 350.0)
      (goto _label)
      (else
        (set `self.ConditionOfRotation` false))))
  (if (`self.ConditionOfRotation`)
    (`SceneComponent.K2_SetRelativeRotation` (`self.CineCamera`) (`KismetMathLibrary.MakeRotator` 0.0 0.0 (`KismetMathLibrary.FClamp` _returnvalue_yaw -2.5 2.5)) false false)))

(fn `UserConstructionScript`)