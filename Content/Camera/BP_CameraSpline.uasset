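; Spline-rail camera actor that follows the player character with a CineCamera.
; Each tick, the camera eases by delta time toward the spline point closest to a position trailing the player along world X, ignoring Y and Z.
; Its rotation blends from the starting rotation toward a look-at on the player, weighted more strongly as the player nears the actor itself, not the moving camera.
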(event `self.ReceiveBeginPlay`
  (set `self.PlayerCharacter` (`GameplayStatics.GetPlayerCharacter` 0))
  (set `self.StartRot` (`SceneComponent.RelativeRotation` (`self.CineCamera`))))

(event `self.ReceiveTick`
  (params (DeltaSeconds :type "Float (single-precision)"))
  (bind _returnvalue (`GameplayStatics.GetPlayerCharacter` 0))
  (bind _cinecamera (`self.CineCamera`))
  (bind _returnvalue_x (`KismetMathLibrary.BreakVector` (`self.K2_GetActorLocation` _returnvalue)))
  (bind _result (`|EaseFunction` "Linear" (`GameplayStatics.GetWorldDeltaSeconds`) (`SceneComponent.K2_GetComponentLocation` _cinecamera) (`SplineComponent.FindLocationClosestToWorldLocation` (`self.Spline`) (`KismetMathLibrary.MakeVector` (+ _returnvalue_x -2000.0)) "World")))
  (bind _output_get (set `self.DistancerToPlayer` (`self.GetDistanceTo` (`ActorComponent.GetOwner` (`self.CineCamera`)) _returnvalue)))
  ;[1 1 1 0.2] Move Camera
  (`SceneComponent.K2_SetWorldLocation` _cinecamera _result false false)
  (`SceneComponent.K2_SetRelativeRotation` (`self.CineCamera`) (`KismetMathLibrary.RLerp` (`self.StartRot`) (`KismetMathLibrary.FindLookAtRotation` _result (`self.K2_GetActorLocation` (`self.PlayerCharacter`))) (`KismetMathLibrary.MapRangeClamped` (`self.DistancerToPlayer`) 4000.0 500.0 0.2 0.8)) false false))

(fn `UserConstructionScript`)