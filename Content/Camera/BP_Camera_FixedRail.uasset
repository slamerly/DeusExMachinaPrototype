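; Fixed-rail camera actor that places a CineCamera along a spline, apparently an unfinished prototype.
; The construction script calls LerpCamera, which maps Range to a distance along the spline and blends yaw between slight opposite angles, keeping pitch and roll.
; Runtime player tracking by closest spline point or border-relative Y is disconnected, the fixed/spline mode setters are empty, and a debug key only prints text.
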(event EventBeginPlay)

(event Collision|EventActorBeginOverlap
  (params (OtherActor :type Actor%20Object%20Reference)))

(event EventTick
  (params (DeltaSeconds :type Float%20%28single-precision%29)))

(event Input|KeyboardEvents|DebugKeyR
  (params (Key :type Key%20Structure :default "None") (ActionValue :type Input%20Action%20Value%20Structure))
  (:Pressed
    (Development|PrintString "Hello")))

(fn ConstructionScript
  (CallFunction|LerpCamera (Variables|Default|GetRange)))

(fn SetFixedCamera)

(fn SetSplineCamera)

(fn LerpCamera
  (params (Range :type Float%20%28double-precision%29))
  (bind _cinecamera (Variables|Default|GetCineCamera))
  (bind _returnvalue (Transformation|GetWorldRotation _cinecamera))
  (Transformation|SetWorldLocation (Variables|Default|GetCineCamera) (.location (Spline|GetTransformatDistanceAlongSpline (Variables|Default|GetSpline) (* Range (Spline|GetSplineLength (Variables|Default|GetSpline))) "World" false)) false false)
  (Transformation|SetWorldRotation _cinecamera (Math|Rotator|Lerp(Rotator) (Math|Rotator|MakeRotator (.roll _returnvalue) (.pitch _returnvalue) -5.0) (Math|Rotator|MakeRotator (.roll _returnvalue) (.pitch _returnvalue) 5.0) Range) false false))