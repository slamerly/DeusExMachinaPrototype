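; Camera actor that snaps its CineCamera along spline points when the player overlaps it.
; BeginPlay caches each spline point's world location.
; On overlap, it picks the highest-X point behind the player on X; the stored pick never resets, so it only advances.
; A timeline then moves the camera from its current location toward a fixed -X offset from that point.
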(event `self.ReceiveBeginPlay`
  (bind _spline (`self.Spline`))
  (for _index (range (`SplineComponent.GetNumberOfSplinePoints` _spline))
    (`KismetArrayLibrary.Array_Add` (`self.SplinePoints Location`) (`SplineComponent.GetLocationAtSplinePoint` _spline _index "World"))
    (set `self.ClosestLocation` (-1e+19 0.0 0.0))))

(event `self.ReceiveActorBeginOverlap`
  (params (OtherActor :type "Actor Object Reference"))
  (cast `/Game/Player/BPC_Player` OtherActor)
  (`self.DetectClosestPoint`))

(event `DetectClosestPoint`
  (bind _closestlocation_x (`KismetMathLibrary.BreakVector` (`self.ClosestLocation`)))
  (bind _returnvalue_x (`KismetMathLibrary.BreakVector` (`self.K2_GetActorLocation` (`GameplayStatics.GetPlayerCharacter` 0))))
  (for _array_element (`self.SplinePoints Location`)
    (if (> _returnvalue_x (.x _array_element))
      (if (> (.x _array_element) _closestlocation_x)
        (set `self.ClosestLocation` (`KismetMathLibrary.MakeVector` (.x _array_element) (.y _array_element) (.z _array_element))))))
  (bind (_direction _newtrack_0) (`Timeline|Timeline` :!via `PlayFromStart`)
    (:`Update`
      (`SceneComponent.K2_SetWorldLocation` (`self.CineCamera`) (`|EaseFunction` "Linear" _newtrack_0 (`SceneComponent.K2_GetComponentLocation` (`self.CineCamera`)) (- (`self.ClosestLocation`) (2500.0 0.0 0.0))) false false))))

(event `self.ReceiveTick`
  (params (DeltaSeconds :type "Float (single-precision)")))

(fn `UserConstructionScript`)