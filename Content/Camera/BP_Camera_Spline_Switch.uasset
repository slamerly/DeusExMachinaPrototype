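; Camera actor that places a CineCamera along a spline, previewed in the editor through its construction script.
; A normalized Range value sets both the camera's distance along the spline and its field of view, interpolated from narrow to wide.
; Only the camera's location follows the spline, not its rotation.
; The fixed/spline camera switch functions are empty stubs, and runtime logic is just a debug key print.
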(event EventBeginPlay)

(event Collision|EventActorBeginOverlap
  (params (OtherActor :type Actor%20Object%20Reference)))

(event EventTick
  (params (DeltaSeconds :type Float%20%28single-precision%29)))

(event Input|KeyboardEvents|DebugKeyR
  (params (Key :type Key%20Structure :default "None") (ActionValue :type Input%20Action%20Value%20Structure))
  (:Pressed
    (Development|PrintString "Hello")))

(fn ConstructionScript
  (Transformation|SetWorldLocation (Variables|Default|GetCineCamera) (.location (Spline|GetTransformatDistanceAlongSpline (Variables|Default|GetSpline) (* (Variables|Default|GetRange) (Spline|GetSplineLength (Variables|Default|GetSpline))) "World" false)) false false)
  (Camera|SetFieldOfView (Variables|Default|GetCineCamera) (Math|Float|Lerp 37.0 65.0 (Variables|Default|GetRange))))

(fn SetFixedCamera)

(fn SetSplineCamera)