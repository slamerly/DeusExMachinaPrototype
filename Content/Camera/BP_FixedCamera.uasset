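; BP_FixedCamera is a fixed camera actor that becomes the player's view target when the player character enters its Box trigger.
; It switches with a configurable blend, from either the overlap event or a delayed BeginPlay check for a player already inside.
; Each switch calls a world camera shake, passing BP_CameraShake at the player's location only when CameraShake is set.
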(event `self.ReceiveBeginPlay`
  (`KismetSystemLibrary.Delay` 0.2)
  (if (`PrimitiveComponent.IsOverlappingActor` (`self.Box`) (`GameplayStatics.GetPlayerCharacter` 0))
    (`self.OnFixedCameraOverlap` :!label _label)
    (if (`self.CameraShake ?`)
      (`GameplayStatics.PlayWorldCameraShake` "/Game/Camera/BP_CameraShake.BP_CameraShake_C" (`SceneComponent.K2_GetComponentLocation` (`Actor.RootComponent` (`GameplayStatics.GetPlayerCharacter` 0))) 0.0 4000.0)
      (else
        (`GameplayStatics.PlayWorldCameraShake` null (0.0 0.0 0.0) 0.0 4000.0)))))

(event `self.Box.OnComponentBeginOverlap`
  (params (OverlappedComponent :type "PrimitiveComponent Object Reference") (OtherActor :type "Actor Object Reference") (OtherComp :type "PrimitiveComponent Object Reference") (OtherBodyIndex :type Integer) (bFromSweep :type Boolean) (SweepResult :type "HitResult Structure (by ref)"))
  (if (== OtherActor (`GameplayStatics.GetPlayerCharacter` 0))
    (goto _label)))

(fn `OnFixedCameraOverlap`
  (`PlayerController.SetViewTargetWithBlend` (`GameplayStatics.GetPlayerController` 0) self (`self.Blend Time`) (`self.Blend Func`) 0.0 false))

(fn `UserConstructionScript`)