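; Act 1 camera actor that becomes the player's view on BeginPlay and pans its CineCamera to follow the player character.
; Tick uses angle hysteresis: rotation starts when the player drifts past a small threshold and stops once nearly centered.
; While rotating it refreshes a flattened target direction, and yaw eases toward it within a clamped range.
; Debug prints remain, and spline-clamped positional lag logic is present but disconnected.
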(event `self.ReceiveBeginPlay`
  (`PlayerController.SetViewTargetWithBlend` (`GameplayStatics.GetPlayerController` 0) self 0.0 "VTBlend_Linear" 0.0 false)
  (set `self.CurrentCamForward` (`KismetMathLibrary.Vector_Normal2D` (`SceneComponent.GetForwardVector` (`self.CineCamera`)))))

(event `self.ReceiveTick`
  (params (DeltaSeconds :type "Float (single-precision)"))
  (bind _cinecamera (`self.CineCamera`))
  (bind _angle_clmap (`self.Angle_Clmap`))
  (bind (_returnvalue_roll _returnvalue_pitch _returnvalue_yaw) (`KismetMathLibrary.BreakRotator` (`KismetMathLibrary.RInterpTo` (`SceneComponent.K2_GetComponentRotation` (`self.CineCamera`)) (`KismetMathLibrary.Conv_VectorToRotator` (`self.CurrentCamForward`)) (`GameplayStatics.GetWorldDeltaSeconds`) 1.5)))
  (set `self.DotProduct` (`KismetMathLibrary.DegAcos` (`KismetMathLibrary.Dot_VectorVector` (`KismetMathLibrary.SelectVector` (`KismetMathLibrary.Vector_Normal2D` (`SceneComponent.GetForwardVector` _cinecamera)) (`self.CurrentCamForward`) (`self.isRotating`)) (`KismetMathLibrary.GetDirectionUnitVector` (`SceneComponent.K2_GetComponentLocation` _cinecamera) (`self.K2_GetActorLocation` (`GameplayStatics.GetPlayerCharacter` 0))))))
  (`KismetSystemLibrary.PrintString` "Hello" true true (struct :`G` 0.66 :`B` 1.0 :`A` 1.0) 0.0 "DotProducttttt")
  (`KismetSystemLibrary.PrintString` (`KismetStringLibrary.Conv_BoolToString` (`self.isRotating`)) true true (struct :`G` 0.66 :`B` 1.0 :`A` 1.0) 0.0 "IsRotating")
  (`SceneComponent.K2_SetRelativeRotation` (`self.CineCamera`) (`KismetMathLibrary.MakeRotator` 0.0 0.0 (`KismetMathLibrary.FClamp` _returnvalue_yaw (* _angle_clmap -1.0) _angle_clmap)) false false)
  (if (`self.isRotating`)
    (set `self.CurrentCamForward` (`KismetMathLibrary.Vector_Normal2D` (`KismetMathLibrary.GetDirectionUnitVector` (`SceneComponent.K2_GetComponentLocation` (`self.CineCamera`)) (`self.K2_GetActorLocation` (`GameplayStatics.GetPlayerCharacter` 0)))))
    (if (`KismetMathLibrary.NearlyEqual_FloatFloat` (`self.DotProduct`) 0.0 1.0)
      (set `self.isRotating` false))
    (elif (> (`self.DotProduct`) 5.0)
      (set `self.isRotating` true))))

(fn `UserConstructionScript`)