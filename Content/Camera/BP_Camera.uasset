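; BP_Camera is a camera actor that becomes the player's view target when play begins.
; A Ctrl+C debug key flip-flops the view between a CameraSpline target and itself with timed blends.
; A transition lock with delays slightly longer than each blend ignores presses mid-transition.
; OnFixedCameraOverlap blends the view back to this camera using configurable time and blend function.
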(event EventBeginPlay
  (Game|Player|SetViewTargetwithBlend (Game|GetPlayerController 0) self 0.0 "VTBlend_Linear" 0.0 false))

(event Input|KeyboardEvents|DebugKeyCtrlC
  (params (Key :type Key%20Structure :default "None") (ActionValue :type Input%20Action%20Value%20Structure))
  (bind _returnvalue (Game|GetPlayerController 0))
  (:Pressed
    (if (not (Variables|Default|GetbCameraTransitionLock))
      (Variables|Default|SetbCameraTransitionLock true)
      (Utilities|FlowControl|FlipFlop
        (:A
          (Game|Player|SetViewTargetwithBlend _returnvalue (Variables|Default|GetCameraSpline) 2.0 "VTBlend_Linear" 0.0 false)
          (Utilities|FlowControl|Delay 2.25)
          (Variables|Default|SetbCameraTransitionLock false))
        (:B
          (Game|Player|SetViewTargetwithBlend _returnvalue self 0.5 "VTBlend_Linear" 0.0 false)
          (Utilities|FlowControl|Delay 0.75)
          (Variables|Default|SetbCameraTransitionLock false))))))

(fn ConstructionScript)

(fn OnFixedCameraOverlap
  (Game|Player|SetViewTargetwithBlend (Game|GetPlayerController 0) self (Variables|Default|GetBlend%20Time) (Variables|Default|GetBlend%20Func) 0.0 false))