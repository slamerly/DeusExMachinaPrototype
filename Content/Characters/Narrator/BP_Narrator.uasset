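; BP_Narrator is the narrator actor, whose mask snaps into a sideways roll at random intervals.
; Tick accumulates and prints a counter, calling TurnHead with a random left or right once it passes a randomized threshold of roughly three seconds.
; TurnHead uses timeline-driven rotator lerps, with a hardcoded branch that always plays the quick timeline, leaving the slow one unused.
; A sine-based vertical movement is present but never runs.
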(event `TurnHead`
  (params (LeftOrRight :type Boolean))
  (bind _returnvalue (`KismetMathLibrary.Conv_BoolToInt` LeftOrRight))
  (if true
    (bind (_direction _alpha) (`Timeline|Rotation_Head_Quick` :!via `PlayFromStart`)
      (:`Update`
        (switch `int` _returnvalue)))
    (else
      (`Timeline|Rotation_Head_Slow` :!via `PlayFromStart`
        (:`Update`
          (switch `int` _returnvalue
            (:`0`
              (`SceneComponent.K2_SetRelativeRotation` (`self.Sm_Mask`) (`KismetMathLibrary.RLerp` (struct) (struct :`Yaw` -90.0) _alpha) false false))
            (:`1`
              (`SceneComponent.K2_SetRelativeRotation` (`self.Sm_Mask`) (`KismetMathLibrary.RLerp` (struct) (struct :`Yaw` 90.0) _alpha) false false))))))))

(event `self.ReceiveTick`
  (params (DeltaSeconds :type "Float (single-precision)"))
  (`|ExecutionSequence`
    (:`then_0`
      (bind _output_get (set `self.Counter` (+ DeltaSeconds (`self.Counter`))))
      (`KismetSystemLibrary.PrintString` (`KismetStringLibrary.Conv_DoubleToString` _output_get) true true (struct :`G` 0.66 :`B` 1.0 :`A` 1.0) 2.0 "Counter")
      (if (> (`self.Counter`) (`KismetMathLibrary.RandomFloatInRange` 2.5 3.5))
        (set `self.Counter` 0.0)
        (`self.TurnHead` (`KismetMathLibrary.RandomBool`))))))

(fn `UserConstructionScript`)